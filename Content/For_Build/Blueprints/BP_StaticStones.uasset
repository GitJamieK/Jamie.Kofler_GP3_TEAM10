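; Static stones actor that stays hidden until activated, then appears as a solid obstacle with a boulder-fall sound.
; BeginPlay turns off the mesh's visibility, collision and component tick.
; The ActivateStaticStones event restores all three and, if CanPlaySoun is set, plays the FMOD BoulderFall event at the actor's location.
; It then releases the sound instance and clears the flag so later activations stay silent.
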(event `self.ReceiveBeginPlay`
  (`SceneComponent.SetVisibility` (`self.StaticMesh`) false false)
  (`PrimitiveComponent.SetCollisionEnabled` (`self.StaticMesh`) "NoCollision")
  (`ActorComponent.SetComponentTickEnabled` (`self.StaticMesh`) false))

(event `ActivateStaticStones`
  (`SceneComponent.SetVisibility` (`self.StaticMesh`) true false)
  (`PrimitiveComponent.SetCollisionEnabled` (`self.StaticMesh`) "QueryAndPhysics")
  (`ActorComponent.SetComponentTickEnabled` (`self.StaticMesh`) true)
  (if (`self.CanPlaySoun`)
    (bind _returnvalue (`FMODBlueprintStatics.PlayEventAtLocation` "/Game/FMOD/Events/Environment/ObjectInteractions/BoulderFall.BoulderFall" (`self.GetTransform`)))
    (`FMODBlueprintStatics.EventInstanceRelease` _returnvalue)
    (set `self.CanPlaySoun` false)))

(fn `UserConstructionScript`)