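; BP_Falling_Rock is a rock prop that drops under physics when its falling event is called.
; The event shows the mesh, waits a random delay, simulates physics for a set duration, then freezes it.
; The first hit, gated by a one-shot flag, plays a boulder-fall audio event at the rock's location and triggers a world camera shake around it.
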(event `Falling Rock event`
  (bind _mesh (`self.Mesh`))
  (`SceneComponent.SetVisibility` (`self.Mesh`) true false)
  (`KismetSystemLibrary.Delay` (`KismetMathLibrary.RandomFloatInRange` 0.1 5.0))
  (`PrimitiveComponent.SetSimulatePhysics` _mesh true)
  (`KismetSystemLibrary.Delay` (`self.Duration`))
  (`PrimitiveComponent.SetSimulatePhysics` _mesh false))

(event `self.Mesh.OnComponentHit`
  (params (HitComponent :type "PrimitiveComponent Object Reference") (OtherActor :type "Actor Object Reference") (OtherComp :type "PrimitiveComponent Object Reference") (NormalImpulse :type "Vector Structure") (Hit :type "HitResult Structure (by ref)"))
  (if (`self.CanPlaySound`)
    (bind _returnvalue (`FMODBlueprintStatics.PlayEventAtLocation` "/Game/FMOD/Events/Environment/ObjectInteractions/BoulderFall.BoulderFall" (`self.GetTransform`)))
    (`FMODBlueprintStatics.EventInstanceRelease` _returnvalue)
    (set `self.CanPlaySound` false)
    (`GameplayStatics.PlayWorldCameraShake` "/Game/Workspaces/GameProgrammers/Galla/BP_FallingRockCameraShake.BP_FallingRockCameraShake_C" (`self.K2_GetActorLocation`) 0.0 3000.0)))

(fn `UserConstructionScript`)