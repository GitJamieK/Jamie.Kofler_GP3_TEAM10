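; BP_Roots is a root prop that switches on its magic material effect when its referenced flower totem is picked up.
; On BeginPlay it binds to the pickup event on the FlowerTotem's GP_FlowerTotemComponent.
; The handler loops over SharedRoot's direct static mesh children, gives material slot 0 a dynamic instance and turns on the MAGIC scalar parameter.
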(event `self.ReceiveBeginPlay`
  (add `GP_FlowerTotemComponent.OnFlowerTotemPickedUp` (`self.GetComponentByClass` (`self.Flower Totem`) "/Script/GP3_TEAM10.GP_FlowerTotemComponent") (delegate `OnFlowerTotemPickedUp_Event`)))

(event `OnFlowerTotemPickedUp_Event`
  (for _array_element (`SceneComponent.GetChildrenComponents` (`self.SharedRoot`) false)
    (bind _asstatic_mesh_component (cast `StaticMeshComponent` _array_element))
    (bind _returnvalue (`PrimitiveComponent.CreateDynamicMaterialInstance` _asstatic_mesh_component 0 (`PrimitiveComponent.GetMaterial` _asstatic_mesh_component 0) "None"))
    (`PrimitiveComponent.SetMaterial` _asstatic_mesh_component 0 _returnvalue)
    (`MaterialInstanceDynamic.SetScalarParameterValue` _returnvalue "MAGIC (0=OFF, 1=ON)" 1.0)))

(fn `UserConstructionScript`)