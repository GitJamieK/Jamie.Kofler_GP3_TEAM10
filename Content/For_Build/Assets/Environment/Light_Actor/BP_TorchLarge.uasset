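; BP_TorchLarge is a torch light actor that flickers by randomizing the intensity of its SpotLight.
; On BeginPlay it starts a Timeline whose updates blend intensity halfway toward TargetIntensity, then pick a new random target after a brief random delay.
; A looping timer, with its period randomized once at start, also calls UpdateTorch to apply the same blend and re-roll the target.
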(event `self.ReceiveBeginPlay`
  (`KismetSystemLibrary.K2_SetTimer` null "UpdateTorch" (`KismetMathLibrary.RandomFloatInRange` 0.2 1.0) true)
  (`Timeline|Timeline`
    (:`Update`
      (`|ExecutionSequence`
        (:`then_0`
          (`LightComponent.SetIntensity` (`self.SpotLight`) (`KismetMathLibrary.Lerp` (`LightComponentBase.Intensity` (`self.SpotLight`)) (`self.Target Intensity`) 0.5)))
        (:`then_1`
          (`KismetSystemLibrary.Delay` (`KismetMathLibrary.RandomFloatInRange` 0.05 0.1))
          (set `self.Target Intensity` (`KismetMathLibrary.RandomFloatInRange` 500.0 2000.0)))))))

(fn `UpdateTorch`
  (`|ExecutionSequence`
    (:`then_0`
      (`LightComponent.SetIntensity` (`self.SpotLight`) (`KismetMathLibrary.Lerp` (`LightComponentBase.Intensity` (`self.SpotLight`)) (`self.Target Intensity`) 0.5)))
    (:`then_1`
      (set `self.Target Intensity` (`KismetMathLibrary.RandomFloatInRange` 500.0 2000.0)))))

(fn `UserConstructionScript`)