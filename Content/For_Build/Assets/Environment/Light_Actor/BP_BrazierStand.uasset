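; BP_BrazierStand is a brazier stand light actor whose spot light flickers in intensity from BeginPlay.
; A Timeline serves as the update tick, with each update moving the light's intensity halfway toward a target value.
; The same update runs a short random Delay, then picks a new random target intensity, so the flicker changes irregularly while staying smoothed.
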(event `self.ReceiveBeginPlay`
  (`Timeline|Timeline`
    (:`Update`
      (`|ExecutionSequence`
        (:`then_0`
          (`LightComponent.SetIntensity` (`self.SpotLight`) (`KismetMathLibrary.Lerp` (`LightComponentBase.Intensity` (`self.SpotLight`)) (`self.Target Intensity`) 0.5)))
        (:`then_1`
          (`KismetSystemLibrary.Delay` (`KismetMathLibrary.RandomFloatInRange` 0.1 0.05))
          (set `self.Target Intensity` (`KismetMathLibrary.RandomFloatInRange` 2000.0 10000.0)))))))

(fn `UserConstructionScript`)