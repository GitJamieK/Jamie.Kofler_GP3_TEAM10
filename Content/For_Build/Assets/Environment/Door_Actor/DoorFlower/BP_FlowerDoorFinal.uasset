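; Flower door exit actor that ends the game with an outro cutscene, then returns to the main menu.
; Picking up the linked flower totem reveals the door's VFX meshes and spotlight and unlocks the exit.
; When the player character then overlaps the box, it calls the game mode's pause handler and shows a video player widget.
; Media player events start playback once the cutscene opens and load the main menu when it ends.
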(event `self.ReceiveBeginPlay`
  (add `GP_FlowerTotemComponent.OnFlowerTotemPickedUp` (`self.GetComponentByClass` (`self.Flower Totem`) "/Script/GP3_TEAM10.GP_FlowerTotemComponent") (delegate `OnFlowerTotemPickedUp_Event`)))

(event `OnFlowerTotemPickedUp_Event`
  (`SceneComponent.SetVisibility` (`self.SM_FlowerDoor_VFX_R`) true false)
  (`SceneComponent.SetVisibility` (`self.SM_FlowerDoor_VFX_L`) true false)
  (`SceneComponent.SetVisibility` (`self.SpotLight`) true false)
  (set `self.CanLeaveThroughDoor` true))

(event `self.Box.OnComponentBeginOverlap`
  (params (OverlappedComponent :type "PrimitiveComponent Object Reference") (OtherActor :type "Actor Object Reference") (OtherComp :type "PrimitiveComponent Object Reference") (OtherBodyIndex :type Integer) (bFromSweep :type Boolean) (SweepResult :type "HitResult Structure (by ref)"))
  (bind _returnvalue (`GameplayStatics.GetPlayerController` 0))
  (bind _returnvalue_2 (`GameplayStatics.GetPlayerController` 0))
  (if (`self.CanLeaveThroughDoor`)
    (cast `/Game/Workspaces/GameProgrammers/Brian/Blueprints/BP_BrianPlayerTestCharacter` OtherActor)
    (bind _asgp_game_mode_base (cast `GP_GameModeBase` (`GameplayStatics.GetGameMode`)))
    (`GP_GameModeBase.HandlePauseState` _asgp_game_mode_base _returnvalue_2)
    (bind _returnvalue_3 (`|CreateWidget` "/Game/UI/WBP_VideoPlayer_Outro.WBP_VideoPlayer_Outro_C" _returnvalue_2))
    (`UserWidget.AddToViewport` _returnvalue_3 0)
    (`WidgetBlueprintLibrary.SetInputMode_GameOnly` _returnvalue)
    (set `PlayerController.bShowMouseCursor` false _returnvalue)
    (`Widget.SetKeyboardFocus` _returnvalue_3)
    (bind _commonvideoplayer_102 (`/Game/UI/WBP_VideoPlayer_Outro.CommonVideoPlayer_102` _returnvalue_3))
    (`CommonVideoPlayer.SetVideo` _commonvideoplayer_102 "/Game/Workspaces/GameDesigners/Leon/Junk/MP4/OutroCutscene.OutroCutscene")
    (`CommonVideoPlayer.SetShouldMatchSize` _commonvideoplayer_102 true)
    (add `MediaPlayer.OnMediaOpened` (`self.MediaPlayer`) (delegate `OnMediaOpened_Event`))
    (add `MediaPlayer.OnEndReached` (`self.MediaPlayer`) (delegate `OnEndReached_Event`))
    (`MediaPlayer.OpenSource` (`self.MediaPlayer`) "/Game/Workspaces/GameDesigners/Leon/Junk/MP4/OutroCutscene.OutroCutscene")))

(event `OnMediaOpened_Event`
  (params (OpenedUrl :type String))
  (`CommonVideoPlayer.Play` (`/Game/UI/WBP_VideoPlayer_Outro.CommonVideoPlayer_102` (stale `self.Box.OnComponentBeginOverlap` _returnvalue_3))))

(event `OnEndReached_Event`
  (`GameplayStatics.OpenLevelBySoftObjectPtr` "/Game/For_Build/Maps/MainMenu/MainMenu.MainMenu"))

(fn `UserConstructionScript`)