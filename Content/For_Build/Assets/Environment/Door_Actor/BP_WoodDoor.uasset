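; Wooden door actor that swings open through the OpenDoor event while its trigger box is flagged occupied.
; A timeline lerps the mesh yaw, with a door sound and collision toggling; it reverses when the player leaves the box.
; Non-AI overlaps show a prompt widget.
; The prompt's creation, pop-up animation and outline depend on IsInBox, which is set only after that function runs.
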(event `Open Door`
  ;[0 0.15 0.05194 0.5] Tech tips
  (if (`self.Is in box`)
    (bind _returnvalue (`FMODBlueprintStatics.PlayEventAtLocation` "/Game/FMOD/Events/Environment/ObjectInteractions/DoorOpen.DoorOpen" (`self.GetTransform`)))
    (`FMODBlueprintStatics.EventInstanceRelease` _returnvalue)
    ;[0 0.15 0.05194 0.5] Tech tips
    (`PrimitiveComponent.SetCollisionEnabled` (`self.SM_Door_Double_A_Solo`) "NoCollision")
    (bind (_direction _openclosedoorcurve) (`Timeline|TL_OpenCloseDoor` :!label _label)
      (:`Update`
        (`SceneComponent.K2_SetRelativeRotation` (`self.SM_Door_Double_A_Solo`) (`KismetMathLibrary.MakeRotator` 0.0 0.0 (`KismetMathLibrary.Lerp` 0.0 (`self.DoorOpenAngle`) _openclosedoorcurve)) false false)))))

(event `self.TV_Door.OnComponentBeginOverlap`
  (params (OverlappedComponent :type "PrimitiveComponent Object Reference") (OtherActor :type "Actor Object Reference") (OtherComp :type "PrimitiveComponent Object Reference") (OtherBodyIndex :type Integer) (bFromSweep :type Boolean) (SweepResult :type "HitResult Structure (by ref)"))
  ;[0 0.15 0.05194 0.5] Tech tips
  (cast `GP_AICharacter` OtherActor
    (:`CastFailed`
      (`|ExecutionSequence`
        (:`then_0`
          (`self.NewFunction`))
        (:`then_1`
          (set `self.Is in box` true)
          (if (== OtherActor (`GameplayStatics.GetPlayerPawn` 0))
            _))))))

(event `self.TV_Door.OnComponentEndOverlap`
  (params (OverlappedComponent :type "PrimitiveComponent Object Reference") (OtherActor :type "Actor Object Reference") (OtherComp :type "PrimitiveComponent Object Reference") (OtherBodyIndex :type Integer))
  ;[0 0.15 0.03569 0.5] Tech tips
  (set `self.Is in box` false)
  (`SceneComponent.SetVisibility` (`self.Widget`) false false)
  (if (== (`GameplayStatics.GetPlayerPawn` 0) OtherActor)
    (bind _returnvalue (`FMODBlueprintStatics.PlayEventAtLocation` "/Game/FMOD/Events/Environment/ObjectInteractions/DoorOpen.DoorOpen" (`self.GetTransform`)))
    (`FMODBlueprintStatics.EventInstanceRelease` _returnvalue)
    ;[0 0.15 0.05194 0.5] Tech tips
    (`PrimitiveComponent.SetCollisionEnabled` (`self.SM_Door_Double_A_Solo`) "QueryOnly")
    (goto _label :!via `Reverse`)))

(event `self.ReceiveBeginPlay`
  (`StaticMeshComponent.SetStaticMesh` (`self.SM_Door_Double_A_Solo`) (`self.DoorStaticMesh`)))

(fn `NewFunction`
  (bind _widget (`self.Widget`))
  (`SceneComponent.SetVisibility` (`self.Widget`) true false)
  (if (`self.Is in box`)
    (bind _returnvalue (`|CreateWidget` "/Game/Workspaces/GameProgrammers/Jamie/Interact/UI_InteractHUD.UI_InteractHUD_C"))
    (bind _output_get (set `self.Interact thing` _returnvalue))
    (`WidgetComponent.SetWidget` _widget _output_get)
    (`SceneComponent.SetVisibility` _widget true false)
    (bind _interact_thing (`self.Interact thing`)
      (:`then`
        (if (`self.Is in box`)
          (`UserWidget.PlayAnimation` _interact_thing (`/Game/Workspaces/GameProgrammers/Jamie/Interact/UI_InteractHUD.PopUp` _interact_thing) 0.0 1 "Forward" 1.5 false)
          (`MeshComponent.SetOverlayMaterial` (`self.Cube`) "/Game/Workspaces/GameProgrammers/Jamie/Materials/M_Outline.M_Outline")))
      (:`else`))))

(fn `UserConstructionScript`)