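; BP_CreepyGate is a double-door gate that slowly swings open when the player pawn enters its trigger volume and closes when it leaves.
; Overlap events play or reverse one timeline, which lerps the yaw of both leaves in opposite directions by DoorOpenAngle.
; BeginPlay applies the DoorStaticMesh variable to both leaves; the construction script is empty.
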(event `self.TV_Door.OnComponentBeginOverlap`
  (params (OverlappedComponent :type "PrimitiveComponent Object Reference") (OtherActor :type "Actor Object Reference") (OtherComp :type "PrimitiveComponent Object Reference") (OtherBodyIndex :type Integer) (bFromSweep :type Boolean) (SweepResult :type "HitResult Structure (by ref)"))
  (if (== OtherActor (`GameplayStatics.GetPlayerPawn` 0))
    (bind (_direction _openclosedoorfloat) (`Timeline|TL_OpenCloseDoorSlow` :!label _label)
      (:`Update`
        (`SceneComponent.K2_SetRelativeRotation` (`self.SM_Door_Double_A_Solo`) (`KismetMathLibrary.MakeRotator` 0.0 0.0 (`KismetMathLibrary.Lerp` 0.0 (- 0.0 (`self.DoorOpenAngle`)) _openclosedoorfloat)) false false)
        (`SceneComponent.K2_SetRelativeRotation` (`self.SM_Door_Double_A_Solo1`) (`KismetMathLibrary.MakeRotator` 0.0 0.0 (`KismetMathLibrary.Lerp` 180.0 (+ (`self.DoorOpenAngle`) 180.0) _openclosedoorfloat)) false false)))))

(event `self.TV_Door.OnComponentEndOverlap`
  (params (OverlappedComponent :type "PrimitiveComponent Object Reference") (OtherActor :type "Actor Object Reference") (OtherComp :type "PrimitiveComponent Object Reference") (OtherBodyIndex :type Integer))
  (if (== (`GameplayStatics.GetPlayerPawn` 0) OtherActor)
    (goto _label :!via `Reverse`)))

(event `self.ReceiveBeginPlay`
  (`StaticMeshComponent.SetStaticMesh` (`self.SM_Door_Double_A_Solo1`) (`self.DoorStaticMesh`))
  (`StaticMeshComponent.SetStaticMesh` (`self.SM_Door_Double_A_Solo`) (`self.DoorStaticMesh`)))

(fn `UserConstructionScript`)