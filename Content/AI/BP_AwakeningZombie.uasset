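; Zombie enemy Blueprint that adds FMOD audio and saved death state to its parent class.
; Construction sets CharacterID from the display name; death records it in the game instance's EnemiesKilled data, and BeginPlay destroys zombies already recorded.
; Idle sounds run on a timer loop with random waits, skipping Sleep and Attack states, then stop after a cooldown; the loop ends on death.
; Damage plays a one-shot sound at the zombie's location.
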(event `self.ReceiveBeginPlay`
  (`self.CheckEnemiesKilled`)
  (`KismetSystemLibrary.K2_SetTimer` null "TryToPlayIdleSound" (`KismetMathLibrary.RandomFloatInRange` (`self.MinIdleSoundWaitTime`) (`self.MaxIdleSoundWaitTime`))))

(event `self.ReceiveTick`
  (params (DeltaSeconds :type "Float (single-precision)"))
  (`parent.ReceiveTick` DeltaSeconds))

(event `self.HealthComponent.OnDamage`
  (params (Damage :type "Float (single-precision)") (DamageType :type "DamageType Object Reference") (InstigatedBy :type "Controller Object Reference"))
  (bind _returnvalue (`FMODBlueprintStatics.PlayEventAtLocation` "/Game/FMOD/Events/Enemies/Zombie/Damaged/ZombieDamaged.ZombieDamaged" (`self.GetTransform`)))
  (`FMODBlueprintStatics.EventInstanceRelease` _returnvalue))

(event `self.HealthComponent.OnDeath`
  (`self.AddToEnemiesKilled`))

(fn `AddToEnemiesKilled`
  (bind _savegamedata (message `/Game/Workspaces/GameProgrammers/Brian/SaveGame/BPI_SaveGame.GetSavedGameData` (`GameplayStatics.GetGameInstance`)))
  (`/Engine/EditorBlueprintResources/StandardMacros.IsValid` _savegamedata
    (:`Is Valid`
      (`BlueprintMapLibrary.Map_Add` (`/Game/Workspaces/GameProgrammers/Brian/SaveGame/BP_SaveGame.EnemiesKilled` _savegamedata) (`self.CharacterID`) true))))

(fn `CheckEnemiesKilled`
  (bind _savegamedata (message `/Game/Workspaces/GameProgrammers/Brian/SaveGame/BPI_SaveGame.GetSavedGameData` (`GameplayStatics.GetGameInstance`)))
  (`/Engine/EditorBlueprintResources/StandardMacros.IsValid` _savegamedata
    (:`Is Valid`
      (if (`BlueprintMapLibrary.Map_Find` (`/Game/Workspaces/GameProgrammers/Brian/SaveGame/BP_SaveGame.EnemiesKilled` _savegamedata) (`self.CharacterID`))
        (`self.K2_DestroyActor`)))))

(fn `ResetIdleSound`
  (`FMODBlueprintStatics.EventInstanceStop` (`self.IdleSoundEvent`) true)
  (set `self.Should Play Idle Sound` true)
  (`KismetSystemLibrary.K2_SetTimer` null "TryToPlayIdleSound" (`KismetMathLibrary.RandomFloatInRange` (`self.MinIdleSoundWaitTime`) (`self.MaxIdleSoundWaitTime`)))
  (return))

(fn `TryToPlayIdleSound`
  (bind _returnvalue (`self.GetCurrentAnimState`))
  (if (`GP_HealthComponent.IsDead` (`self.HealthComponent`))
    _
    (elif (and (`|EnumInequality` _returnvalue "Sleep") (`|EnumInequality` _returnvalue "Attack"))
      (if (`self.Should Play Idle Sound`)
        (set `self.Should Play Idle Sound` false)
        (bind _returnvalue_2 (`FMODBlueprintStatics.PlayEventAtLocation` "/Game/FMOD/Events/Enemies/Zombie/Idle/ZombieIdle.ZombieIdle" (`self.GetTransform`)))
        (set `self.IdleSoundEvent` _returnvalue_2)
        (`KismetSystemLibrary.K2_SetTimer` null "ResetIdleSound" (`self.Idle Fmod Sound Cooldown`)))
      (else
        (`KismetSystemLibrary.K2_SetTimer` null "TryToPlayIdleSound" (`KismetMathLibrary.RandomFloatInRange` (`self.MinIdleSoundWaitTime`) (`self.MaxIdleSoundWaitTime`)))))))

(fn `UserConstructionScript`
  (set `self.CharacterID` (`KismetSystemLibrary.GetDisplayName` self)))