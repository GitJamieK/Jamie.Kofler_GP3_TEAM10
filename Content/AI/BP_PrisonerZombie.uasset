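; Prisoner zombie enemy that handles its FMOD voice audio and stays dead through saved game data.
; Randomized timers alternate between playing and resetting the idle sound, which pauses briefly for a damage sound while alive and stops for the death sound.
; On death it records its display-name-based CharacterID in the saved EnemiesKilled map, and on BeginPlay destroys itself if already listed there.
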(event `self.ReceiveBeginPlay`
  (`self.CheckEnemiesKilled`)
  (`KismetSystemLibrary.K2_SetTimer` null "TryToPlayIdleSound" (`KismetMathLibrary.RandomFloatInRange` (`self.MinIdleSoundWaitTime`) (`self.MaxIdleSoundWaitTime`))))

(event `self.HealthComponent.OnDamage`
  (params (Damage :type "Float (single-precision)") (DamageType :type "DamageType Object Reference") (InstigatedBy :type "Controller Object Reference"))
  (if (> (`GP_HealthComponent.GetHealth` (`self.HealthComponent`)) 0.0)
    (`FMODBlueprintStatics.EventInstanceSetPaused` (`self.IdleSoundEvent`) true)
    (bind _returnvalue (`FMODBlueprintStatics.PlayEventAtLocation` "/Game/FMOD/Events/Enemies/Zombie/Damaged/ZombieDamaged.ZombieDamaged" (`self.GetTransform`)))
    (`FMODBlueprintStatics.EventInstanceRelease` _returnvalue)
    (`KismetSystemLibrary.Delay` (`KismetMathLibrary.RandomFloatInRange` 1.0 2.0))
    (`FMODBlueprintStatics.EventInstanceSetPaused` (`self.IdleSoundEvent`))))

(event `self.HealthComponent.OnDeath`
  (`FMODBlueprintStatics.EventInstanceStop` (`self.IdleSoundEvent`) true)
  (bind _returnvalue (`FMODBlueprintStatics.PlayEventAtLocation` "/Game/FMOD/Events/Enemies/Zombie/Death/ZombieDeath.ZombieDeath" (`self.GetTransform`)))
  (`FMODBlueprintStatics.EventInstanceRelease` _returnvalue)
  (`self.AddToEnemiesKilled`))

(fn `AddToEnemiesKilled`
  (bind _savegamedata (message `/Game/Workspaces/GameProgrammers/Brian/SaveGame/BPI_SaveGame.GetSavedGameData` (`GameplayStatics.GetGameInstance`)))
  (`/Engine/EditorBlueprintResources/StandardMacros.IsValid` _savegamedata
    (:`Is Valid`
      (`BlueprintMapLibrary.Map_Add` (`/Game/Workspaces/GameProgrammers/Brian/SaveGame/BP_SaveGame.EnemiesKilled` _savegamedata) (`self.CharacterID`) true))))

(fn `CheckEnemiesKilled`
  (bind _savegamedata (message `/Game/Workspaces/GameProgrammers/Brian/SaveGame/BPI_SaveGame.GetSavedGameData` (`GameplayStatics.GetGameInstance`)))
  (`/Engine/EditorBlueprintResources/StandardMacros.IsValid` _savegamedata
    (:`Is Valid`
      (if (`BlueprintMapLibrary.Map_Find` (`/Game/Workspaces/GameProgrammers/Brian/SaveGame/BP_SaveGame.EnemiesKilled` _savegamedata) (`self.CharacterID`))
        (`self.K2_DestroyActor`)))))

(fn `ResetIdleSound`
  (`FMODBlueprintStatics.EventInstanceStop` (`self.IdleSoundEvent`) true)
  (set `self.ShouldPlayIdleSound` true)
  (`KismetSystemLibrary.K2_SetTimer` null "TryToPlayIdleSound" (`KismetMathLibrary.RandomFloatInRange` (`self.MinIdleSoundWaitTime`) (`self.MaxIdleSoundWaitTime`)))
  (return))

(fn `TryToPlayIdleSound`
  (if (`GP_HealthComponent.IsDead` (`self.HealthComponent`))
    _
    (elif (`self.ShouldPlayIdleSound`)
      (set `self.ShouldPlayIdleSound` false)
      (bind _returnvalue (`FMODBlueprintStatics.PlayEventAtLocation` "/Game/FMOD/Events/Enemies/Zombie/Idle/ZombieIdle.ZombieIdle" (`self.GetTransform`)))
      (set `self.IdleSoundEvent` _returnvalue)
      (`KismetSystemLibrary.K2_SetTimer` null "ResetIdleSound" (`self.IdleFmodSoundCooldown`)))))

(fn `UserConstructionScript`
  (set `self.CharacterID` (`KismetSystemLibrary.GetDisplayName` self)))