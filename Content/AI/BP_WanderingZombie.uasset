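; Wandering zombie AI character that adds FMOD audio for idle and damage feedback.
; On Tick, after the parent logic, it plays a one-shot idle sound at its location while alive, gated by a flag that a cooldown timer resets.
; Health component damage events trigger a one-shot hurt sound at the zombie's position.
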(event `self.ReceiveTick`
  (params (DeltaSeconds :type "Float (single-precision)"))
  (`parent.ReceiveTick` DeltaSeconds)
  (if (`GP_HealthComponent.IsDead` (`self.HealthComponent`))
    _
    (elif (`self.bShouldPlayIdleSound`)
      (set `self.bShouldPlayIdleSound` false)
      (bind _returnvalue (`FMODBlueprintStatics.PlayEventAtLocation` "/Game/FMOD/Events/Enemies/Zombie/Idle/ZombieIdle.ZombieIdle" (`self.GetTransform`)))
      (`FMODBlueprintStatics.EventInstanceRelease` _returnvalue)
      (`KismetSystemLibrary.K2_SetTimer` null "ResetIdleSound" (`self.Idle Fmod Sound Cooldown`)))))

(event `self.HealthComponent.OnDamage`
  (params (Damage :type "Float (single-precision)") (DamageType :type "DamageType Object Reference") (InstigatedBy :type "Controller Object Reference"))
  (bind _returnvalue (`FMODBlueprintStatics.PlayEventAtLocation` "/Game/FMOD/Events/Enemies/Zombie/Damaged/ZombieDamaged.ZombieDamaged" (`self.GetTransform`)))
  (`FMODBlueprintStatics.EventInstanceRelease` _returnvalue))

(fn `ResetIdleSound`
  (set `self.bShouldPlayIdleSound` true)
  (return))

(fn `UserConstructionScript`)