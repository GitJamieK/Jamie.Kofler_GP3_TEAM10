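; BP_tutorial is a tutorial trigger that updates the player's tutorial widget when BP_BackupDorukCharacter overlaps its Box.
; On overlap, it calls GetAwayUI(true) on the character's TutorialWidget and fills two text fields from its own text variables.
; It then clears CanActivate so the trigger fires only once, and calls GetAwayUI(false) after a long fixed delay.
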(event `self.Box.OnComponentBeginOverlap`
  (params (OverlappedComponent :type "PrimitiveComponent Object Reference") (OtherActor :type "Actor Object Reference") (OtherComp :type "PrimitiveComponent Object Reference") (OtherBodyIndex :type Integer) (bFromSweep :type Boolean) (SweepResult :type "HitResult Structure (by ref)"))
  (if (`self.CanActivate`)
    (bind _asbp_backup_doruk_character (cast `/Game/Workspaces/GameProgrammers/Doruk/Blueprints/BP_BackupDorukCharacter` OtherActor))
    (bind _tutorialwidget (`/Game/Workspaces/GameProgrammers/Doruk/Blueprints/BP_BackupDorukCharacter.TutorialWidget` _asbp_backup_doruk_character))
    (`/Game/Workspaces/GameDesigners/Leon/Leon_UI/WBP_tutorial.Get away UI` _tutorialwidget true)
    (set `MultiLineEditableText.Text` (`self.Normal Text`) (`/Game/Workspaces/GameDesigners/Leon/Leon_UI/WBP_tutorial.NormalText` _tutorialwidget))
    (set `MultiLineEditableText.Text` (`self.Normal Text_0`) (`/Game/Workspaces/GameDesigners/Leon/Leon_UI/WBP_tutorial.NormalText1` _tutorialwidget))
    (set `self.CanActivate` false)
    (`KismetSystemLibrary.Delay` 50.0)
    (`/Game/Workspaces/GameDesigners/Leon/Leon_UI/WBP_tutorial.Get away UI` _tutorialwidget false)))

(fn `UserConstructionScript`)