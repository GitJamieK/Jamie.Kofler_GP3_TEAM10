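; Candle prop with a point light that flickers like a flame, starting on BeginPlay.
; Each Timeline update moves the light intensity halfway toward a target value.
; The same update triggers a short random Delay, after which a new random target intensity is picked, producing a smoothed, irregular flicker.
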(event `self.ReceiveBeginPlay`
  (`Timeline|Timeline`
    (:`Update`
      (`|ExecutionSequence`
        (:`then_0`
          (`LightComponent.SetIntensity` (`self.PointLight`) (`KismetMathLibrary.Lerp` (`LightComponentBase.Intensity` (`self.PointLight`)) (`self.Target Intensity`) 0.5)))
        (:`then_1`
          (`KismetSystemLibrary.Delay` (`KismetMathLibrary.RandomFloatInRange` 0.05 0.1))
          (set `self.Target Intensity` (`KismetMathLibrary.RandomFloatInRange` 10.0 20.0)))))))

(fn `UserConstructionScript`)