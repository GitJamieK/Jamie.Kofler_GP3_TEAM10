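; Falling platform that breaks away when its trigger box is overlapped and stays gone once recorded as passed.
; Overlap enables physics on the cube, then after a short delay removes a second box, enables gravity on the GCCube15 piece and plays a boulder-fall sound event.
; It later saves its ID, taken from the display name in the construction script, and destroys itself; BeginPlay destroys platforms already saved.
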(event `self.ReceiveBeginPlay`
  (bind _savegamedata (message `/Game/Workspaces/GameProgrammers/Brian/SaveGame/BPI_SaveGame.GetSavedGameData` (`GameplayStatics.GetGameInstance`)))
  (`/Engine/EditorBlueprintResources/StandardMacros.IsValid` _savegamedata
    (:`Is Valid`
      (if (`BlueprintMapLibrary.Map_Find` (`/Game/Workspaces/GameProgrammers/Brian/SaveGame/BP_SaveGame.FallingPlatformsPassed` _savegamedata) (`self.FallingPlatformID`))
        (`self.K2_DestroyActor`)))))

(event `self.Box.OnComponentBeginOverlap`
  (params (OverlappedComponent :type "PrimitiveComponent Object Reference") (OtherActor :type "Actor Object Reference") (OtherComp :type "PrimitiveComponent Object Reference") (OtherBodyIndex :type Integer) (bFromSweep :type Boolean) (SweepResult :type "HitResult Structure (by ref)"))
  (`PrimitiveComponent.SetSimulatePhysics` (`self.Cube`) true)
  (`KismetSystemLibrary.Delay` 0.9)
  (`ActorComponent.K2_DestroyComponent` (`self.Box1`))
  (`PrimitiveComponent.SetEnableGravity` (`self.GC_Cube15`) true)
  (bind _returnvalue (`FMODBlueprintStatics.PlayEventAtLocation` "/Game/FMOD/Events/Environment/ObjectInteractions/BoulderFall.BoulderFall" (`self.GetTransform`)))
  (`FMODBlueprintStatics.EventInstanceRelease` _returnvalue)
  (`KismetSystemLibrary.Delay` 3.0)
  (bind _savegamedata (message `/Game/Workspaces/GameProgrammers/Brian/SaveGame/BPI_SaveGame.GetSavedGameData` (`GameplayStatics.GetGameInstance`)))
  (`/Engine/EditorBlueprintResources/StandardMacros.IsValid` _savegamedata
    (:`Is Valid`
      (`BlueprintMapLibrary.Map_Add` (`/Game/Workspaces/GameProgrammers/Brian/SaveGame/BP_SaveGame.FallingPlatformsPassed` _savegamedata) (`self.FallingPlatformID`) true)
      (`self.K2_DestroyActor`))))

(fn `UserConstructionScript`
  (set `self.FallingPlatformID` (`KismetSystemLibrary.GetDisplayName` self)))