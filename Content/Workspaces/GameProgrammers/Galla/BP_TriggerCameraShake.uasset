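; Trigger volume that plays a one-shot flower event camera shake once the flower totem has been picked up.
; On BeginPlay it binds to the FlowerTotem's component pickup delegate, which sets a flag.
; A later box overlap by the player character plays a world camera shake with radial falloff, centered on the first player controller's location, then destroys the actor.
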(event `self.ReceiveBeginPlay`
  (add `GP_FlowerTotemComponent.OnFlowerTotemPickedUp` (`self.GetComponentByClass` (`self.FlowerTotem`) "/Script/GP3_TEAM10.GP_FlowerTotemComponent") (delegate `OnFlowerTotemPickedUp_Event`)))

(event `OnFlowerTotemPickedUp_Event`
  (set `self.IsFlowerPickedUp` true))

(event `self.BoxTrigger.OnComponentBeginOverlap`
  (params (OverlappedComponent :type "PrimitiveComponent Object Reference") (OtherActor :type "Actor Object Reference") (OtherComp :type "PrimitiveComponent Object Reference") (OtherBodyIndex :type Integer) (bFromSweep :type Boolean) (SweepResult :type "HitResult Structure (by ref)"))
  (if (`self.IsFlowerPickedUp`)
    (cast `GP_PlayerCharacter` OtherActor
      (:`then`
        (`GameplayStatics.PlayWorldCameraShake` "/Game/Workspaces/GameProgrammers/Galla/BP_FlowerEventCameraShake.BP_FlowerEventCameraShake_C" (`self.K2_GetActorLocation` (`GameplayStatics.GetPlayerController` 0)) 0.0 500.0 1.0 true)
        (`self.K2_DestroyActor`))
      (:`CastFailed`
        (`KismetSystemLibrary.PrintString` "FAILED CAST")))))

(fn `UserConstructionScript`)