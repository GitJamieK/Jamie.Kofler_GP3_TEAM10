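; Temporary flower totem that the player picks once while inside its sphere trigger, starting an escape sequence.
; Interact triggers falling rocks and static stones, plays the pick montage with a movement lock, then grants a temporary key item and destroys the flower with camera shake and sound.
; It then pauses the game for a fullscreen pickup cutscene, using media player callbacks to remove it, unpause and start escape music.
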(event `self.ReceiveBeginPlay`
  (set `self.Starting Rotation` (`SceneComponent.RelativeRotation` (`self.StaticMesh`)))
  (set `self.IsInBox` false))

(event `/Game/Workspaces/GameProgrammers/Jamie/Interact/BPI_Interaction.Interact`
  (bind _returnvalue (`GameplayStatics.GetPlayerController` 0))
  (bind _returnvalue_2 (`GameplayStatics.GetPlayerController` 0))
  (if (`self.IsInBox`)
    (if (not (`self.IsFlowerPickedUp`))
      (`|ExecutionSequence`
        (:`then_0`
          (bind _outactors (`GameplayStatics.GetAllActorsOfClass` "/Game/For_Build/Blueprints/BP_Falling_Rock.BP_Falling_Rock_C"))
          (`/Game/For_Build/Blueprints/BP_Falling_Rock.Falling Rock event` _outactors)
          (bind _asbp_brian_player_test_character (cast `/Game/Workspaces/GameProgrammers/Brian/Blueprints/BP_BrianPlayerTestCharacter` (stale `self.Sphere.OnComponentBeginOverlap` OtherActor)))
          (if (`self.CanInteract`)
            (`/Game/Workspaces/GameProgrammers/Doruk/Blueprints/BP_BackupDorukCharacter.PlayAnimationMontage` _asbp_brian_player_test_character "/Game/For_Build/Animations/Player_Misc_Montage.Player_Misc_Montage" "Pick")
            (`/Game/Workspaces/GameProgrammers/Doruk/Blueprints/BP_BackupDorukCharacter.LockMovement` _asbp_brian_player_test_character 1.2)
            ; Added Delay For Animation To Look Good
            (`KismetSystemLibrary.Delay` 0.5)
            (`GP_InventoryComponent.AddItem` (`/Game/Workspaces/GameProgrammers/Brian/Blueprints/BP_BrianPlayerTestCharacter.GP_Inventory` _asbp_brian_player_test_character) "KeyTEMP" 1 0)
            (set `self.CanInteract` false)
            (`GP_FlowerTotemComponent.OnPickedUp_Implementation` (`self.GP_FlowerTotem`))
            (`GameplayStatics.PlayWorldCameraShake` "/Game/Workspaces/GameProgrammers/Galla/BP_FlowerEventCameraShake.BP_FlowerEventCameraShake_C" (`self.K2_GetActorLocation` (`GameplayStatics.GetPlayerController` 0)) 0.0 500.0 1.0 true)
            (`ActorComponent.K2_DestroyComponent` (`self.flower`))
            (`SceneComponent.SetHiddenInGame` (`self.Widget`) true false)
            (set `self.IsFlowerPickedUp` true)
            (bind _returnvalue_3 (`FMODBlueprintStatics.PlayEventAtLocation` "/Game/FMOD/Events/Environment/ObjectInteractions/FlowerPickup.FlowerPickup" (`self.GetTransform`)))
            (`FMODBlueprintStatics.EventInstanceRelease` _returnvalue_3)
            (bind _asgp_game_mode_base (cast `GP_GameModeBase` (`GameplayStatics.GetGameMode`)))
            (`GP_GameModeBase.HandlePauseState` _asgp_game_mode_base _returnvalue_2)
            (bind _returnvalue_4 (`|CreateWidget` "/Game/UI/WBP_VideoPlayer_FlowerPickup.WBP_VideoPlayer_FlowerPickup_C" _returnvalue_2))
            (`UserWidget.AddToViewport` _returnvalue_4 0)
            (`WidgetBlueprintLibrary.SetInputMode_GameOnly` _returnvalue)
            (set `PlayerController.bShowMouseCursor` false _returnvalue)
            (`Widget.SetKeyboardFocus` _returnvalue_4)
            (bind _commonvideoplayer_102 (`/Game/UI/WBP_VideoPlayer_FlowerPickup.CommonVideoPlayer_102` _returnvalue_4))
            (`CommonVideoPlayer.SetVideo` _commonvideoplayer_102 "/Game/Workspaces/GameDesigners/Leon/Junk/MP4/FlowerPickupCutscene.FlowerPickupCutscene")
            (`CommonVideoPlayer.SetShouldMatchSize` _commonvideoplayer_102 true)
            (add `MediaPlayer.OnMediaOpened` (`self.MediaPlayer`) (delegate `OnMediaOpened_Event`))
            (add `MediaPlayer.OnEndReached` (`self.MediaPlayer`) (delegate `OnEndReached_Event`))
            (`MediaPlayer.OpenSource` (`self.MediaPlayer`) "/Game/Workspaces/GameDesigners/Leon/Junk/MP4/FlowerPickupCutscene.FlowerPickupCutscene")))
        (:`then_1`
          (bind _outactors_2 (`GameplayStatics.GetAllActorsOfClass` "/Game/For_Build/Blueprints/BP_StaticStones.BP_StaticStones_C"))
          (`/Game/For_Build/Blueprints/BP_StaticStones.ActivateStaticStones` _outactors_2))))))

(event `OnMediaOpened_Event`
  (params (OpenedUrl :type String))
  (`CommonVideoPlayer.Play` (`/Game/UI/WBP_VideoPlayer_FlowerPickup.CommonVideoPlayer_102` (stale `/Game/Workspaces/GameProgrammers/Jamie/Interact/BPI_Interaction.Interact` _returnvalue_4))))

(event `self.Sphere.OnComponentBeginOverlap`
  (params (OverlappedComponent :type "PrimitiveComponent Object Reference") (OtherActor :type "Actor Object Reference") (OtherComp :type "PrimitiveComponent Object Reference") (OtherBodyIndex :type Integer) (bFromSweep :type Boolean) (SweepResult :type "HitResult Structure (by ref)"))
  (set `self.IsInBox` true))

(event `self.Can Receive Trace`
  (params (`Can Interact` :type Boolean)))

(event `OnEndReached_Event`
  (`Widget.RemoveFromParent` (stale `/Game/Workspaces/GameProgrammers/Jamie/Interact/BPI_Interaction.Interact` _returnvalue_4))
  (bind _asgp_game_mode_base (cast `GP_GameModeBase` (`GameplayStatics.GetGameMode`)))
  (`GP_GameModeBase.HandleUnPauseState` _asgp_game_mode_base)
  (`KismetSystemLibrary.Delay` 1.0)
  (`FMODBlueprintStatics.PlayEvent2D` "/Game/FMOD/Events/Music/EscapeMusic.EscapeMusic"))

(event `self.Sphere.OnComponentEndOverlap`
  (params (OverlappedComponent :type "PrimitiveComponent Object Reference") (OtherActor :type "Actor Object Reference") (OtherComp :type "PrimitiveComponent Object Reference") (OtherBodyIndex :type Integer))
  (set `self.IsInBox` false))

(fn `UserConstructionScript`
  (`parent.UserConstructionScript`))