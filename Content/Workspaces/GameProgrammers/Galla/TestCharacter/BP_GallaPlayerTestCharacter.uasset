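; Test player character Blueprint that routes the interact input between quick-time events and item interaction.
; On interact, it calls OnQTEButtonPressed when the GP_GameModeBase gameplay state is QTEState; otherwise, or if the cast fails, it sends InteractMessage through TraceItem.
; GetAttackPoint returns the skeletal mesh's world transform.
; Debug prints remain, and a QTE-start chain calling HandleQTEState is left unconnected.
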(event `EnhancedInput|/Game/Workspaces/GameProgrammers/Doruk/Input/Actions/IA_CC_Interact`
  (params (ActionValue :type Boolean) (ElapsedSeconds :type "Float (double-precision)") (TriggeredSeconds :type "Float (double-precision)") (InputAction :type "InputAction Object Reference" :default "/Game/Workspaces/GameProgrammers/Doruk/Input/Actions/IA_CC_Interact.IA_CC_Interact"))
  (:`Triggered`
    (bind _asgp_game_mode_base (cast `GP_GameModeBase` (`GameplayStatics.GetGameMode`))
      (:`then`
        (`KismetSystemLibrary.PrintString` "qqqqqq")
        (if (`|EnumEquality` (`GP_GameModeBase.GetGameplayState` _asgp_game_mode_base) "QTEState")
          (`self.OnQTEButtonPressed`)
          (`KismetSystemLibrary.PrintString` "Hello")
          (else
            (`KismetSystemLibrary.PrintString` "fuuck")
            (message `/Game/Workspaces/GameProgrammers/Jamie/Interact/BPI_Interaction.Interact` (`self.Trace Item`) :!label _label))))
      (:`CastFailed`
        (goto _label)))))

(fn `GetAttackPoint`
  (returns (ReturnValue :type "Transform Structure"))
  (return (`SceneComponent.K2_GetComponentToWorld` (`self.SkeletalMesh`))))

(fn `UserConstructionScript`
  (`parent.UserConstructionScript`))