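; Test player character that turns health changes into HUD and camera feedback and hands death to the game mode.
; A timeline lerps the health bar, desaturation and vignette, then toggles bar visibility and starts a ping-pong vignette pulse at low health.
; F spends an inventory health pack to heal, and T applies test damage to itself.
; AimWeapon switches walk speed and fades the crosshair and ammo switcher widgets.
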(event `self.ReceiveBeginPlay`
  (`parent.ReceiveBeginPlay`)
  (add `GP_HealthComponent.OnDeath` (`self.GP_Health`) (delegate `OnDeath_Event`))
  (`self.ChangeHPBarVisibility`))

(event `OnDeath_Event`
  (bind _asgp_game_mode_base (cast `GP_GameModeBase` (`GameplayStatics.GetGameMode`)))
  (`GP_GameModeBase.HandleDeathState` _asgp_game_mode_base))

(event `self.GP_Health.OnHealthChanged`
  (params (Health :type "Float (single-precision)") (Delta :type "Float (single-precision)"))
  (bind _returnvalue (`GP_HealthComponent.GetHealthPercent` (`self.GP_Health`)))
  (bind ((`ColorSaturation` _colorsaturation) (`VignetteIntensity` _vignetteintensity)) (break `PostProcessSettings` (`CameraComponent.PostProcessSettings` (`self.FollowCamera`))))
  (bind ((`ColorSaturation` _colorsaturation_2) (`VignetteIntensity` _vignetteintensity_2)) (break `PostProcessSettings` (`CameraComponent.PostProcessSettings` (`self.FollowCamera`))))
  ; Logic of Post Processing Changes Based on HP
  (bind (_direction _smoothfloatcurve) (`Timeline|TL_SmoothPostProcess` :!via `PlayFromStart`)
    (:`Update`
      (`self.ChangeHPBar` Health Delta _smoothfloatcurve)
      (set `CameraComponent.PostProcessSettings` (make `PostProcessSettings` :`ColorSaturation` (`KismetMathLibrary.MakeVector4` 1.0 1.0 1.0 (`KismetMathLibrary.Lerp` (`.W` (`KismetMathLibrary.BreakVector4` _colorsaturation)) _returnvalue _smoothfloatcurve)) :`VignetteIntensity` (`KismetMathLibrary.Lerp` _vignetteintensity (+ (- 1.0 _returnvalue) 0.1) _smoothfloatcurve)) (`self.FollowCamera`)))
    (:`Finished`
      (`self.ChangeHPBarVisibility`)
      (if (<= (`GP_HealthComponent.GetHealthPercent` (`self.GP_Health`)) 0.2)
        (bind (_direction_2 _lerpvalue) (`Timeline|TL_PulsatingVignette` :!via `PlayFromStart` :!label _label)
          (:`Update`
            (switch `ETimelineDirection` _direction_2
              (:`Forward`
                (set `CameraComponent.PostProcessSettings` (make `PostProcessSettings` :`ColorSaturation` (`KismetMathLibrary.MakeVector4` 1.0 1.0 1.0 (`.W` (`KismetMathLibrary.BreakVector4` _colorsaturation_2))) :`VignetteIntensity` (`KismetMathLibrary.Lerp` _vignetteintensity_2 (+ _vignetteintensity_2 0.02) _lerpvalue)) (`self.FollowCamera`)))
              (:`Backward`
                (set `CameraComponent.PostProcessSettings` (make `PostProcessSettings` :`ColorSaturation` (`KismetMathLibrary.MakeVector4` 1.0 1.0 1.0 (`.W` (`KismetMathLibrary.BreakVector4` _colorsaturation_2))) :`VignetteIntensity` (`KismetMathLibrary.Lerp` (- _vignetteintensity_2 0.02) _vignetteintensity_2 _lerpvalue)) (`self.FollowCamera`)))))
          (:`Finished`
            (`/Engine/EditorBlueprintResources/StandardMacros.FlipFlop`
              (:`A`
                (goto _label :!via `ReverseFromEnd`))
              (:`B`
                (goto _label :!via `PlayFromStart`)))))
        (else
          (goto _label :!via `Stop`))))))

(event `Key|F`
  (params (Key :type "Key Structure"))
  ; Heal Logic
  (:`Pressed`
    (if (`GP_HealthComponent.IsHealthFull` (`self.GP_Health`))
      (`KismetSystemLibrary.PrintString` "You're Full HP!!" true true (struct :`R` 1.0 :`B` 0.139721 :`A` 1.0))
      (else
        (bind _returnvalue (`GP_InventoryComponent.UseItem` (`self.GP_Inventory`) "HealthPack"))
        (if _returnvalue
          (`GP_HealthComponent.TryToAddHealth` (`self.GP_Health`) 50.0)
          (else
            (`KismetSystemLibrary.PrintString` "No Health Packs!" true true (struct :`R` 1.0 :`G` 0.082806 :`B` 0.072858 :`A` 1.0))))))))

(event `Key|T`
  (params (Key :type "Key Structure"))
  ;[1 0 0 0.5] Testing
  (:`Pressed`
    (`GameplayStatics.ApplyDamage` self 10.0)))

(fn `AimWeapon`
  (params (bIsAiming :type Boolean))
  (if bIsAiming
    (`self.PlayFadeInAnim`)
    (set `CharacterMovementComponent.MaxWalkSpeed` (`self.PlayerAimingSpeed`) (`self.CharacterMovement`))
    (else
      (`self.PlayFadeOutAnim`)
      (set `CharacterMovementComponent.MaxWalkSpeed` (`self.PlayerWalkingSpeed`) (`self.CharacterMovement`))))
  (return))

(fn `ChangeHPBar`
  (params (NewHealth :type "Float (double-precision)") (HealthChanged :type "Float (double-precision)") (LerpFloat :type "Float (double-precision)"))
  (bind _asgame_hud (cast `/Game/UI/GameHUD` (`PlayerController.GetHUD` (`GameplayStatics.GetPlayerController` 0))))
  (`ProgressBar.SetPercent` (`/Game/UI/WBP_HealthBar.HPBar` (`/Game/UI/GameHUD.UI_HealthBarRef` _asgame_hud)) (/ (`KismetMathLibrary.Lerp` (- NewHealth HealthChanged) NewHealth LerpFloat) 100.0)))

(fn `ChangeHPBarVisibility`
  (bind _returnvalue (`GP_HealthComponent.IsHealthFull` (`self.GP_Health`)))
  (bind _asgame_hud (cast `/Game/UI/GameHUD` (`PlayerController.GetHUD` (`GameplayStatics.GetPlayerController` 0))))
  (bind _ui_healthbarref (`/Game/UI/GameHUD.UI_HealthBarRef` _asgame_hud))
  (bind (_colorandopacity_r _colorandopacity_g _colorandopacity_b _colorandopacity_a) (break `LinearColor` (`UserWidget.ColorAndOpacity` _ui_healthbarref)))
  (bind _returnvalue_2 (== 0.0 _colorandopacity_a))
  (if _returnvalue_2
    (if (!= _returnvalue_2 _returnvalue)
      (bind _fadeinout (`/Game/UI/WBP_HealthBar.FadeInOut` _ui_healthbarref))
      (`UserWidget.PlayAnimation` _ui_healthbarref _fadeinout 0.0 1 "Forward" 1.0 false))
    (elif _returnvalue
      (`UserWidget.PlayAnimation` _ui_healthbarref _fadeinout 0.0 1 "Reverse" 1.0 false))))

(fn `PlayFadeInAnim`
  (bind _asgame_hud (cast `/Game/UI/GameHUD` (`PlayerController.GetHUD` (`GameplayStatics.GetPlayerController` 0))))
  (bind _ui_ammoswitcherref (`/Game/UI/GameHUD.UI_AmmoSwitcherRef` _asgame_hud))
  (`UserWidget.PlayAnimation` _ui_ammoswitcherref (`/Game/UI/AmmoUI/WBP_AmmoSwitcher.Fade` _ui_ammoswitcherref) 0.0 1 "Forward" 1.0 false)
  (bind _ui_crosshairref (`/Game/UI/GameHUD.UI_CrosshairRef` _asgame_hud))
  (`UserWidget.PlayAnimation` _ui_crosshairref (`/Game/UI/WBP_Crosshair.Fade` _ui_crosshairref) 0.0 1 "Forward" 1.0 false))

(fn `PlayFadeOutAnim`
  (bind _asgame_hud (cast `/Game/UI/GameHUD` (`PlayerController.GetHUD` (`GameplayStatics.GetPlayerController` 0))))
  (bind _ui_ammoswitcherref (`/Game/UI/GameHUD.UI_AmmoSwitcherRef` _asgame_hud))
  (`UserWidget.PlayAnimation` _ui_ammoswitcherref (`/Game/UI/AmmoUI/WBP_AmmoSwitcher.Fade` _ui_ammoswitcherref) 0.0 1 "Reverse" 1.0 false)
  (bind _ui_crosshairref (`/Game/UI/GameHUD.UI_CrosshairRef` _asgame_hud))
  (`UserWidget.PlayAnimation` _ui_crosshairref (`/Game/UI/WBP_Crosshair.Fade` _ui_crosshairref) 0.0 1 "Reverse" 1.0 false))

(fn `UserConstructionScript`
  (`parent.UserConstructionScript`))