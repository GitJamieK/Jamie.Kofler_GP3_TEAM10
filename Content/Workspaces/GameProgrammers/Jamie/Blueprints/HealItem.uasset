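; A heal item Blueprint that the player interacts with and that destroys itself on use.
; On begin play it stores the static mesh's relative rotation, which nothing in the graph uses afterwards.
; Interact requires both CanPressE and CanInteract, then clears CanInteract and destroys the actor through an always-true branch.
; No healing logic appears in this graph.
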(event `self.ReceiveBeginPlay`
  (set `self.Starting Rotation` (`SceneComponent.RelativeRotation` (`self.StaticMesh`))))

(event `/Game/Workspaces/GameProgrammers/Jamie/Interact/BPI_Interaction.Interact`
  (if (`self.CanPressE`)
    (if (`self.CanInteract`)
      (set `self.CanInteract` false)
      (if true
        (`self.K2_DestroyActor`)))))

(fn `UserConstructionScript`
  (`parent.UserConstructionScript`))