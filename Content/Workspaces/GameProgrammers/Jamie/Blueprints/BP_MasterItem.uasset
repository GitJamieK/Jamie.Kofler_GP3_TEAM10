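; Base pickup item Blueprint that shows an interaction prompt and stays gone once collected.
; Sphere overlap with the player character toggles CanInteract and an animated widget prompt, choosing its button icon by current input type.
; The picked-up delegate records ItemID, taken from the display name at construction, in the GameInstance's saved data; BeginPlay destroys items already recorded there.
; Interact is empty here, and the outline overlay logic is disconnected.
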(event `self.ReceiveBeginPlay`
  (add `self.PickedUpItem` (delegate `CE_UpdatePickedUpItemsDictionary`))
  (bind _savegamedata (message `/Game/Workspaces/GameProgrammers/Brian/SaveGame/BPI_SaveGame.GetSavedGameData` (`GameplayStatics.GetGameInstance`)))
  (`/Engine/EditorBlueprintResources/StandardMacros.IsValid` _savegamedata
    (:`Is Valid`
      (if (`BlueprintMapLibrary.Map_Find` (`/Game/Workspaces/GameProgrammers/Brian/SaveGame/BP_SaveGame.ItemsPickedUp` _savegamedata) (`self.ItemID`))
        (`self.K2_DestroyActor`)))))

(event `CE_UpdatePickedUpItemsDictionary` :!signature `self.PickedUpItem`
  (params (ItemType :type "EItemType Enum" :default "None") (ItemAmount :type Integer))
  (bind _savegamedata (message `/Game/Workspaces/GameProgrammers/Brian/SaveGame/BPI_SaveGame.GetSavedGameData` (`GameplayStatics.GetGameInstance`)))
  (`/Engine/EditorBlueprintResources/StandardMacros.IsValid` _savegamedata
    (:`Is Valid`
      (`BlueprintMapLibrary.Map_Add` (`/Game/Workspaces/GameProgrammers/Brian/SaveGame/BP_SaveGame.ItemsPickedUp` _savegamedata) (`self.ItemID`) true)
      (`KismetSystemLibrary.PrintString` "Item Picked Up!"))))

(event `self.Sphere.OnComponentBeginOverlap`
  (params (OverlappedComponent :type "PrimitiveComponent Object Reference") (OtherActor :type "Actor Object Reference") (OtherComp :type "PrimitiveComponent Object Reference") (OtherBodyIndex :type Integer) (bFromSweep :type Boolean) (SweepResult :type "HitResult Structure (by ref)"))
  (cast `GP_AICharacter` OtherActor
    (:`CastFailed`
      (cast `/Game/Workspaces/GameProgrammers/Brian/Blueprints/BP_BrianPlayerTestCharacter` OtherActor)
      (`self.ShowWidget`))))

(event `self.Sphere.OnComponentEndOverlap`
  (params (OverlappedComponent :type "PrimitiveComponent Object Reference") (OtherActor :type "Actor Object Reference") (OtherComp :type "PrimitiveComponent Object Reference") (OtherBodyIndex :type Integer))
  (cast `/Game/Workspaces/GameProgrammers/Brian/Blueprints/BP_BrianPlayerTestCharacter` OtherActor)
  (`self.HideWidget`))

(event `/Game/Workspaces/GameProgrammers/Jamie/Interact/BPI_Interaction.Can Receive Trace`
  (params (`Can Interact` :type Boolean))
  (if (`self.CanInteract`)
    (if `Can Interact`
      (bind _interaction_widget (`self.Interaction Widget`)
        (:`then`
          (if (not (`self.ButtonVisible`))
            (`UserWidget.PlayAnimation` _interaction_widget (`/Game/Workspaces/GameProgrammers/Jamie/Interact/UI_InteractHUD.PopUp` _interaction_widget) 0.0 1 "Forward" 1.5 false)
            (set `self.ButtonVisible` true)))
        (:`else`))
      (else
        (bind _interaction_widget_2 (`self.Interaction Widget`)
          (:`then`
            (if (`self.ButtonVisible`)
              (`UserWidget.PlayAnimation` _interaction_widget_2 (`/Game/Workspaces/GameProgrammers/Jamie/Interact/UI_InteractHUD.PopUp` _interaction_widget_2) 0.0 1 "Reverse" 1.5 false)
              (set `self.ButtonVisible` false)))
          (:`else`))))))

(event `/Game/Workspaces/GameProgrammers/Jamie/Interact/BPI_Interaction.Interact`)

(fn `HideWidget`
  (bind _interaction_widget (`self.Interaction Widget`)
    (:`then`
      (if (`self.ButtonVisible`)
        (`UserWidget.PlayAnimation` _interaction_widget (`/Game/Workspaces/GameProgrammers/Jamie/Interact/UI_InteractHUD.PopUp` _interaction_widget) 0.0 1 "Reverse" 1.5 false)
        (set `self.ButtonVisible` false))
      (`Widget.RemoveFromParent` (`self.Interaction Widget`))
      (set `self.Interaction Widget` null)
      (`SceneComponent.SetVisibility` (`self.Widget`) false false)
      (set `self.CanInteract` false))
    (:`else`)))

(fn `ShowWidget`
  (bind _widget (`self.Widget`))
  (bind _returnvalue (`|GetEnumeratorNameAsString` (`CommonInputSubsystem.GetCurrentInputType` (pcsubsystem `CommonInputSubsystem` (`GameplayStatics.GetPlayerController` 0)))))
  (bind _returnvalue_2 (`|CreateWidget` "/Game/Workspaces/GameProgrammers/Jamie/Interact/UI_InteractHUD.UI_InteractHUD_C"))
  (bind _output_get (set `self.Interaction Widget` _returnvalue_2))
  (`WidgetComponent.SetWidget` _widget _output_get)
  (`KismetSystemLibrary.PrintString` _returnvalue)
  (if (`KismetStringLibrary.EqualEqual_StrStr` _returnvalue "Mouse And Keyboard")
    (bind _buttonswitcher (`/Game/Workspaces/GameProgrammers/Jamie/Interact/UI_InteractHUD.ButtonSwitcher` _output_get))
    (`WidgetSwitcher.SetActiveWidgetIndex` _buttonswitcher 1)
    (else
      (`WidgetSwitcher.SetActiveWidgetIndex` _buttonswitcher 0)))
  (`SceneComponent.SetVisibility` _widget true false)
  (bind _interaction_widget (`self.Interaction Widget`)
    (:`then`
      (if (not (`self.ButtonVisible`))
        (`UserWidget.PlayAnimation` _interaction_widget (`/Game/Workspaces/GameProgrammers/Jamie/Interact/UI_InteractHUD.PopUp` _interaction_widget) 0.0 1 "Forward" 1.5 false)
        (set `self.ButtonVisible` true)
        (set `self.CanInteract` true)))
    (:`else`)))

(fn `UserConstructionScript`
  (set `self.ItemID` (`KismetSystemLibrary.GetDisplayName` self)))