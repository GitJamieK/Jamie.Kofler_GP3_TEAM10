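; Temporary health pickup that heals the player character when interacted with.
; Interact is gated by CanPressE and CanInteract, then calls TryToAddHealth on the GP_HealthComponent of BP_JamiePlayerCharacter with a fixed amount.
; On success it prints a debug message and destroys itself; CanInteract is cleared before the attempt and not restored here if healing fails.
; BeginPlay caches the mesh's starting rotation, which this graph never reads.
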(event `self.ReceiveBeginPlay`
  (set `self.Starting Rotation` (`SceneComponent.RelativeRotation` (`self.StaticMesh`))))

(event `/Game/Workspaces/GameProgrammers/Jamie/Interact/BPI_Interaction.Interact`
  (if (`self.CanPressE`)
    (if (`self.CanInteract`)
      (set `self.CanInteract` false)
      (if true
        (bind _asbp_jamie_player_character (cast `/Game/Workspaces/GameProgrammers/Jamie/Blueprints/BP_JamiePlayerCharacter` (`GameplayStatics.GetPlayerCharacter` 0)))
        (bind _returnvalue (`GP_HealthComponent.TryToAddHealth` (`self.GetComponentByClass` _asbp_jamie_player_character "/Script/GP3_TEAM10.GP_HealthComponent") 20.0))
        (if _returnvalue
          (`KismetSystemLibrary.PrintString` "Added Health")
          (`self.K2_DestroyActor`))))))

(fn `UserConstructionScript`
  (`parent.UserConstructionScript`))