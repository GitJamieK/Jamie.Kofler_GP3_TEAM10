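; Readable paper note that shows its narrative and hint text in a WBP_NotePickupWidget on screen.
; Interact and sphere begin-overlap share one path that, for BP_BrianPlayerTestCharacter, opens the note with a MenuMove audio event if allowed, or puts it down if already reading.
; AlejandrosTexts fills the widget from the note's text variables.
; Leaving the sphere also removes the widget and resets the reading state.
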(event `self.ReceiveBeginPlay`
  (set `self.Starting Rotation` (`SceneComponent.RelativeRotation` (`self.StaticMesh`)))
  (set `self.IsNotReading` true))

(event `/Game/Workspaces/GameProgrammers/Jamie/Interact/BPI_Interaction.Interact`
  (cast `/Game/Workspaces/GameProgrammers/Brian/Blueprints/BP_BrianPlayerTestCharacter` (stale `self.Sphere.OnComponentBeginOverlap` OtherActor) :!label _label)
  (if (and (`self.CanInteract`) (`self.IsNotReading`))
    (`self.Alejandros Texts`)
    (set `self.IsNotReading` false)
    (`FMODBlueprintStatics.PlayEventAtLocation` "/Game/FMOD/Events/UI/Menu/MenuMove.MenuMove" (`self.GetTransform`))
    (elif (not (`self.IsNotReading`))
      (`self.PutDownNote`))))

(event `self.Sphere.OnComponentBeginOverlap`
  (params (OverlappedComponent :type "PrimitiveComponent Object Reference") (OtherActor :type "Actor Object Reference") (OtherComp :type "PrimitiveComponent Object Reference") (OtherBodyIndex :type Integer) (bFromSweep :type Boolean) (SweepResult :type "HitResult Structure (by ref)"))
  (goto _label))

(event `self.Sphere.OnComponentEndOverlap`
  (params (OverlappedComponent :type "PrimitiveComponent Object Reference") (OtherActor :type "Actor Object Reference") (OtherComp :type "PrimitiveComponent Object Reference") (OtherBodyIndex :type Integer))
  (bind _papernote (`self.PaperNote`))
  ; Puts down note when leaving area
  (cast `/Game/Workspaces/GameProgrammers/Brian/Blueprints/BP_BrianPlayerTestCharacter` OtherActor)
  (if (`KismetSystemLibrary.IsValid` _papernote)
    (`Widget.RemoveFromParent` _papernote)
    (set `self.IsNotReading` true)))

(event `PutDownNote`
  ; EVENT  - putting down note when interacting again
  (if (`self.IsNotReading`)
    _
    (elif (`KismetSystemLibrary.IsValid` (`self.PaperNote`))
      (`Widget.RemoveFromParent` (`self.PaperNote`))
      (set `self.IsNotReading` true)
      (set `self.CanInteract` true))))

(event `Alejandro's E Press`)

(event `Alejandros Texts`
  ;[0.04026 0 0.15 0.5] Narrative Scripting
  (bind _returnvalue (`|CreateWidget` "/Game/Workspaces/GameDesigners/Alejandro/BluePrints/WBP_NotePickupWidget.WBP_NotePickupWidget_C"))
  (bind _output_get (set `self.PaperNote` _returnvalue))
  (set `MultiLineEditableText.Text` (`self.Normal Text`) (`/Game/Workspaces/GameDesigners/Alejandro/BluePrints/WBP_NotePickupWidget.NormalText` _output_get))
  (set `MultiLineEditableText.Text` (`self.Name Text`) (`/Game/Workspaces/GameDesigners/Alejandro/BluePrints/WBP_NotePickupWidget.NameText` _output_get))
  (set `MultiLineEditableText.Text` (`self.Year Text`) (`/Game/Workspaces/GameDesigners/Alejandro/BluePrints/WBP_NotePickupWidget.YearText` _output_get))
  (set `MultiLineEditableText.Text` (`self.Hint Normal Text`) (`/Game/Workspaces/GameDesigners/Alejandro/BluePrints/WBP_NotePickupWidget.HintNormalText` _output_get))
  (set `MultiLineEditableText.Text` (`self.Hint Name Text`) (`/Game/Workspaces/GameDesigners/Alejandro/BluePrints/WBP_NotePickupWidget.HintNameText` _output_get))
  (set `MultiLineEditableText.Text` (`self.Hint Year Text`) (`/Game/Workspaces/GameDesigners/Alejandro/BluePrints/WBP_NotePickupWidget.HintYearTExt` _output_get))
  (`UserWidget.AddToViewport` _output_get 0))

(fn `UserConstructionScript`
  (`parent.UserConstructionScript`))