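; Temporary ammo pickup item that the player interacts with, currently a stub that grants no ammo.
; On BeginPlay it stores the static mesh's starting rotation.
; Interact prints a debug message and destroys the actor when CanInteract is set, otherwise it reports the player is too far away.
; CanReceiveTrace is empty, and a player component lookup is left unconnected.
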(event `self.ReceiveBeginPlay`
  (set `self.Starting Rotation` (`SceneComponent.RelativeRotation` (`self.StaticMesh`))))

(event `/Game/Workspaces/GameProgrammers/Jamie/Interact/BPI_Interaction.Interact`
  (if (`self.CanInteract`)
    (if true
      (`KismetSystemLibrary.PrintString` "PRESSED AMMO" true true (struct :`G` 0.66 :`B` 1.0 :`A` 1.0) 5.0)
      (set `self.CanInteract` false)
      (`self.K2_DestroyActor`))
    (else
      (`KismetSystemLibrary.PrintString` "Too far to interact!" true true (struct :`R` 1.0 :`B` 0.031298 :`A` 1.0)))))

(event `/Game/Workspaces/GameProgrammers/Jamie/Interact/BPI_Interaction.Can Receive Trace`
  (params (`Can Interact` :type Boolean)))

(fn `UserConstructionScript`
  (`parent.UserConstructionScript`))