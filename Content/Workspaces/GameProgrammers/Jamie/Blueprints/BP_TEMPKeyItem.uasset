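; Temporary key pickup actor that the player can interact with to collect a key.
; When CanInteract is true, Interact adds one KeyTEMP to the BP_BrianPlayerTestCharacter's GPInventory and destroys the actor, otherwise it prints a too-far message.
; BeginPlay caches the mesh's starting rotation, which nothing here reads, and CanReceiveTrace is an empty event.
; This file never sets CanInteract to true.
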(event `self.ReceiveBeginPlay`
  (set `self.Starting Rotation` (`SceneComponent.RelativeRotation` (`self.StaticMesh`))))

(event `/Game/Workspaces/GameProgrammers/Jamie/Interact/BPI_Interaction.Interact`
  (if (`self.CanInteract`)
    (bind _asbp_brian_player_test_character (cast `/Game/Workspaces/GameProgrammers/Brian/Blueprints/BP_BrianPlayerTestCharacter` (`GameplayStatics.GetPlayerCharacter` 0)))
    (`GP_InventoryComponent.AddItem` (`/Game/Workspaces/GameProgrammers/Brian/Blueprints/BP_BrianPlayerTestCharacter.GP_Inventory` _asbp_brian_player_test_character) "KeyTEMP" 1 0)
    (set `self.CanInteract` false)
    (`self.K2_DestroyActor`)
    (else
      (`KismetSystemLibrary.PrintString` "Too far to interact!" true true (struct :`R` 1.0 :`B` 0.031298 :`A` 1.0)))))

(event `/Game/Workspaces/GameProgrammers/Jamie/Interact/BPI_Interaction.Can Receive Trace`
  (params (`Can Interact` :type Boolean)))

(fn `UserConstructionScript`
  (`parent.UserConstructionScript`))