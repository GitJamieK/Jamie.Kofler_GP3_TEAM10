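; Temporary shotgun ammo pickup that adds ammo to the Brian test character's inventory.
; Interact and sphere overlap share one path, which casts the overlap's OtherActor and checks CanInteract.
; It plays a pick montage and locks movement, with a short delay before adding ammo to suit the animation.
; It then disables interaction, calls PickedUpItem, plays a released one-shot pickup sound event and destroys itself.
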(event `self.ReceiveBeginPlay`
  (set `self.Starting Rotation` (`SceneComponent.RelativeRotation` (`self.StaticMesh`)))
  (`parent.ReceiveBeginPlay`))

(event `/Game/Workspaces/GameProgrammers/Jamie/Interact/BPI_Interaction.Interact`
  (bind _ammotoadd (`self.AmmoToAdd`))
  (bind _asbp_brian_player_test_character (cast `/Game/Workspaces/GameProgrammers/Brian/Blueprints/BP_BrianPlayerTestCharacter` (stale `self.Sphere.OnComponentBeginOverlap` OtherActor) :!label _label))
  (if (`self.CanInteract`)
    (`/Game/Workspaces/GameProgrammers/Doruk/Blueprints/BP_BackupDorukCharacter.PlayAnimationMontage` _asbp_brian_player_test_character "/Game/For_Build/Animations/Player_Misc_Montage.Player_Misc_Montage" "Pick")
    (`/Game/Workspaces/GameProgrammers/Doruk/Blueprints/BP_BackupDorukCharacter.LockMovement` _asbp_brian_player_test_character 1.2)
    ; Added Delay For Animation To Look Good
    (`KismetSystemLibrary.Delay` 0.5)
    (`GP_InventoryComponent.AddItem` (`/Game/Workspaces/GameProgrammers/Brian/Blueprints/BP_BrianPlayerTestCharacter.GP_Inventory` _asbp_brian_player_test_character) "ShotgunAmmo" _ammotoadd 0)
    (set `self.CanInteract` false)
    (`self.PickedUpItem` "ShotgunAmmo" _ammotoadd)
    (bind _returnvalue (`FMODBlueprintStatics.PlayEventAtLocation` "/Game/FMOD/Events/Environment/ObjectInteractions/FirePickup.FirePickup" (`self.GetTransform`)))
    (`FMODBlueprintStatics.EventInstanceRelease` _returnvalue)
    (`self.K2_DestroyActor`)))

(event `self.Sphere.OnComponentBeginOverlap`
  (params (OverlappedComponent :type "PrimitiveComponent Object Reference") (OtherActor :type "Actor Object Reference") (OtherComp :type "PrimitiveComponent Object Reference") (OtherBodyIndex :type Integer) (bFromSweep :type Boolean) (SweepResult :type "HitResult Structure (by ref)"))
  (goto _label))

(fn `UserConstructionScript`
  (`parent.UserConstructionScript`))