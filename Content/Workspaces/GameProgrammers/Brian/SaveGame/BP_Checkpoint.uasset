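; Checkpoint actor that saves the game once, when the test player character enters its trigger area.
; After a short delay, the overlap passes the player's save data and the checkpoint's reached state to the Game Instance for synchronous saving.
; The construction script derives CheckpointID from the actor's display name, and BeginPlay uses it to restore the triggered state from saved data.
; An unconnected branch holds GameMode-based respawn snapshot logic.
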(event `self.ReceiveBeginPlay`
  (bind _savegamedata (message `/Game/Workspaces/GameProgrammers/Brian/SaveGame/BPI_SaveGame.GetSavedGameData` (`GameplayStatics.GetGameInstance`)))
  (`/Engine/EditorBlueprintResources/StandardMacros.IsValid` _savegamedata
    (:`Is Valid`
      (set `self.WasTriggeredBefore` (`BlueprintMapLibrary.Map_Find` (`/Game/Workspaces/GameProgrammers/Brian/SaveGame/BP_SaveGame.CheckpointsReached` _savegamedata) (`self.CheckpointID`))))))

(event `self.CheckpointArea.OnComponentBeginOverlap`
  (params (OverlappedComponent :type "PrimitiveComponent Object Reference") (OtherActor :type "Actor Object Reference") (OtherComp :type "PrimitiveComponent Object Reference") (OtherBodyIndex :type Integer) (bFromSweep :type Boolean) (SweepResult :type "HitResult Structure (by ref)"))
  (`KismetSystemLibrary.Delay` 0.2)
  (bind _asbp_brian_player_test_character (cast `/Game/Workspaces/GameProgrammers/Brian/Blueprints/BP_BrianPlayerTestCharacter` OtherActor))
  (if (not (`self.WasTriggeredBefore`))
    (set `self.WasTriggeredBefore` true)
    (bind _playersave (`/Game/Workspaces/GameProgrammers/Brian/Blueprints/BP_BrianPlayerTestCharacter.GetPlayerSaveData` _asbp_brian_player_test_character))
    (message `/Game/Workspaces/GameProgrammers/Brian/SaveGame/BPI_SaveGame.SavePlayer` (`GameplayStatics.GetGameInstance`) _playersave false)
    (message `/Game/Workspaces/GameProgrammers/Brian/SaveGame/BPI_SaveGame.SaveCheckpoint` (`GameplayStatics.GetGameInstance`) (`self.CheckpointID`) true false)))

(fn `UserConstructionScript`
  (set `self.CheckpointID` (`KismetSystemLibrary.GetDisplayName` self)))