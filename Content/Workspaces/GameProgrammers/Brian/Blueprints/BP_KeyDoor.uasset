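; Puzzle door that sinks open after three keys have been used at key pillars, and stays open through saved game data.
; On BeginPlay it binds to the used-key event of every BP_KeyPillarBase, and CheckKeys counts uses.
; Opening plays a metal gate sound and a timeline lerp downward, then records the door's display-name ID as passed.
; Doors already recorded as passed are lowered immediately on BeginPlay.
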(event `self.ReceiveBeginPlay`
  (bind _defaultsceneroot (`self.DefaultSceneRoot`))
  (bind (_returnvalue_x _returnvalue_y _returnvalue_z) (`KismetMathLibrary.BreakVector` (`SceneComponent.K2_GetComponentLocation` _defaultsceneroot)))
  (`self.BindUsedKey`)
  (bind _savegamedata (message `/Game/Workspaces/GameProgrammers/Brian/SaveGame/BPI_SaveGame.GetSavedGameData` (`GameplayStatics.GetGameInstance`)))
  (`/Engine/EditorBlueprintResources/StandardMacros.IsValid` _savegamedata
    (:`Is Valid`
      (if (`BlueprintMapLibrary.Map_Find` (`/Game/Workspaces/GameProgrammers/Brian/SaveGame/BP_SaveGame.KeyDoorsPassed` _savegamedata) (`self.KeyDoorID`))
        (`SceneComponent.K2_SetRelativeTransform` _defaultsceneroot (`KismetMathLibrary.MakeTransform` (`KismetMathLibrary.MakeVector` _returnvalue_x _returnvalue_y (- _returnvalue_z 250.0)) (`SceneComponent.K2_GetComponentRotation` _defaultsceneroot)) false false)))))

(event `CE_OpenPuzzleDoor`
  (bind _defaultsceneroot (`self.DefaultSceneRoot`))
  (bind (_returnvalue_x _returnvalue_y _returnvalue_z) (`KismetMathLibrary.BreakVector` (`SceneComponent.K2_GetComponentLocation` _defaultsceneroot)))
  (bind _returnvalue (`FMODBlueprintStatics.PlayEventAtLocation` "/Game/FMOD/Events/Environment/ObjectInteractions/MetalGate.MetalGate" (`self.GetTransform`)))
  (`FMODBlueprintStatics.EventInstanceRelease` _returnvalue)
  (bind (_direction _lerpvalue) (`Timeline|TL_OpenPuzzleDoor`)
    (:`Update`
      (`SceneComponent.K2_SetRelativeTransform` _defaultsceneroot (`KismetMathLibrary.MakeTransform` (`KismetMathLibrary.MakeVector` _returnvalue_x _returnvalue_y (`KismetMathLibrary.Lerp` _returnvalue_z (- _returnvalue_z 250.0) _lerpvalue)) (`SceneComponent.K2_GetComponentRotation` _defaultsceneroot)) false false))
    (:`Finished`
      (bind _savegamedata (message `/Game/Workspaces/GameProgrammers/Brian/SaveGame/BPI_SaveGame.GetSavedGameData` (`GameplayStatics.GetGameInstance`)))
      (`/Engine/EditorBlueprintResources/StandardMacros.IsValid` _savegamedata
        (:`Is Valid`
          (`BlueprintMapLibrary.Map_Add` (`/Game/Workspaces/GameProgrammers/Brian/SaveGame/BP_SaveGame.KeyDoorsPassed` _savegamedata) (`self.KeyDoorID`) true))))))

(fn `BindUsedKey`
  (bind _outactors (`GameplayStatics.GetAllActorsOfClass` "/Game/Workspaces/GameProgrammers/Brian/Blueprints/BP_KeyPillarBase.BP_KeyPillarBase_C"))
  (for _array_element _outactors
    (add `/Game/Workspaces/GameProgrammers/Brian/Blueprints/BP_KeyPillarBase.UsedKey` _array_element (`|CreateDelegate` :!event `CheckKeys`))))

(fn `CheckKeys`
  (params (KeyType :type "EItemType Enum" :default "None"))
  (bind _result (`/Engine/EditorBlueprintResources/StandardMacros.IncrementInt` (`self.KeysUsed`))
    (:`  `
      (if (== _result 3)
        (`self.CE_OpenPuzzleDoor`)))))

(fn `UserConstructionScript`
  (set `self.KeyDoorID` (`KismetSystemLibrary.GetDisplayName` self)))