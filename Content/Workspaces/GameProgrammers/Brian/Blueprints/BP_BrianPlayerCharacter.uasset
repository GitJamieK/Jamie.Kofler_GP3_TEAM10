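; Player character Blueprint, apparently a programmer's workspace variant, that gives visual feedback for health through the follow camera.
; When the health component reports a change, it rebuilds the camera's post-process settings, lowering saturation and raising vignette intensity as health percent drops.
; A test key applies damage to the character itself to exercise the effect.
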(event `self.GP_Health.OnHealthChanged`
  (params (Health :type "Float (single-precision)") (Delta :type "Float (single-precision)"))
  (bind _returnvalue (`GP_HealthComponent.GetHealthPercent` (`self.GP_Health`)))
  (set `CameraComponent.PostProcessSettings` (make `PostProcessSettings` :`ColorSaturation` (`KismetMathLibrary.MakeVector4` 1.0 1.0 1.0 _returnvalue) :`VignetteIntensity` (+ (- 1.0 _returnvalue) 0.4)) (`self.FollowCamera`)))

(event `Key|T`
  (params (Key :type "Key Structure"))
  ;[1 0 0 0.5] Testing
  (:`Pressed`
    (`GameplayStatics.ApplyDamage` self 10.0)))

(fn `UserConstructionScript`
  (`parent.UserConstructionScript`))