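; Damageable puzzle trigger that fires its lock-triggered call when damaged while the player holds weapon index 0.
; Triggering shows the fire effect, zeroes health, records completion in saved game data and plays a break sound; other weapons cause health to be refilled.
; BeginPlay restores the triggered state from that save data, keyed by an ID the construction script takes from the actor's display name.
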(event `self.GP_Health.OnDamage`
  (params (Damage :type "Float (single-precision)") (DamageType :type "DamageType Object Reference") (InstigatedBy :type "Controller Object Reference"))
  (bind _gp_health (`self.GP_Health`))
  (bind _asbp_brian_player_test_character (cast `/Game/Workspaces/GameProgrammers/Brian/Blueprints/BP_BrianPlayerTestCharacter` (`GameplayStatics.GetPlayerCharacter` 0)))
  (if (== (`/Game/Workspaces/GameProgrammers/Doruk/Blueprints/BP_BackupDorukCharacter.CurrentWeaponIndex` _asbp_brian_player_test_character) 0)
    (`self.LockTriggered`)
    (`SceneComponent.SetVisibility` (`self.NS_Fire`) true false)
    (`GP_HealthComponent.SetHealth` (`self.GP_Health`) 0.0)
    (bind _savegamedata (message `/Game/Workspaces/GameProgrammers/Brian/SaveGame/BPI_SaveGame.GetSavedGameData` (`GameplayStatics.GetGameInstance`)))
    (`/Engine/EditorBlueprintResources/StandardMacros.IsValid` _savegamedata
      (:`Is Valid`
        (`BlueprintMapLibrary.Map_Add` (`/Game/Workspaces/GameProgrammers/Brian/SaveGame/BP_SaveGame.PuzzleTriggersDone` _savegamedata) (`self.PuzzleTriggerID`) true)
        (bind _returnvalue (`FMODBlueprintStatics.PlayEventAtLocation` "/Game/FMOD/Events/Environment/ObjectInteractions/TargetBreak.TargetBreak" (`self.GetTransform`)))
        (`FMODBlueprintStatics.EventInstanceRelease` _returnvalue)))
    (else
      (bind _returnvalue_2 (`GP_HealthComponent.TryToAddHealth` _gp_health (- (`GP_HealthComponent.MaxHealth` _gp_health) (`GP_HealthComponent.GetHealth` _gp_health))))
      (if (not _returnvalue_2)
        (`KismetSystemLibrary.PrintString` "Couldn't restore HP to the PuzzleTrigger!" true true (struct :`R` 0.257671 :`G` 0.103803 :`B` 1.0 :`A` 1.0))))))

(event `self.ReceiveBeginPlay`
  (bind _savegamedata (message `/Game/Workspaces/GameProgrammers/Brian/SaveGame/BPI_SaveGame.GetSavedGameData` (`GameplayStatics.GetGameInstance`)))
  (`/Engine/EditorBlueprintResources/StandardMacros.IsValid` _savegamedata
    (:`Is Valid`
      (if (`BlueprintMapLibrary.Map_Find` (`/Game/Workspaces/GameProgrammers/Brian/SaveGame/BP_SaveGame.PuzzleTriggersDone` _savegamedata) (`self.PuzzleTriggerID`))
        (`self.LockTriggered`)
        (`SceneComponent.SetVisibility` (`self.NS_Fire`) true false)
        (`GP_HealthComponent.SetHealth` (`self.GP_Health`) 0.0)
        (else
          (`SceneComponent.SetVisibility` (`self.NS_Fire`) false false))))))

(fn `UserConstructionScript`
  (set `self.PuzzleTriggerID` (`KismetSystemLibrary.GetDisplayName` self)))