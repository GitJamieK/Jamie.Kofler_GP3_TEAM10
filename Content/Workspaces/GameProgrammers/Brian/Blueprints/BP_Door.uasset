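; BP_Door is a puzzle door that slides vertically open once its assigned lock triggers have fired.
; On BeginPlay it binds to the LockTriggered event of each actor in PuzzleTriggerActors.
; CheckLocks counts triggers, calling the open event when the count equals the array length.
; A timeline curve then lerps the root's Z between fixed values, so the height is not offset from the placed position.
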(event `self.ReceiveBeginPlay`
  (`self.BindLockTriggered`))

(event `CE_OpenDoor`
  (bind _defaultsceneroot (`self.DefaultSceneRoot`))
  (bind (_returnvalue_x _returnvalue_y) (`KismetMathLibrary.BreakVector` (`SceneComponent.K2_GetComponentLocation` _defaultsceneroot)))
  (bind (_direction _openclosedoorcurve) (`Timeline|TL_OpenDoor`)
    (:`Update`
      (`SceneComponent.K2_SetRelativeTransform` _defaultsceneroot (`KismetMathLibrary.MakeTransform` (`KismetMathLibrary.MakeVector` _returnvalue_x _returnvalue_y (`KismetMathLibrary.Lerp` 0.0 250.0 _openclosedoorcurve))) false false))))

(fn `BindLockTriggered`
  (for _array_element (`self.PuzzleTriggerActors`)
    (add `/Game/Workspaces/GameProgrammers/Brian/Blueprints/BP_PuzzleTrigger.LockTriggered` _array_element (`|CreateDelegate` :!event `CheckLocks`))))

(fn `CheckLocks`
  (bind _result (`/Engine/EditorBlueprintResources/StandardMacros.IncrementInt` (`self.LocksTriggered`))
    (:`  `
      (if (== _result (`KismetArrayLibrary.Array_Length` (`self.PuzzleTriggerActors`)))
        (`self.CE_OpenDoor`)))))

(fn `UserConstructionScript`)