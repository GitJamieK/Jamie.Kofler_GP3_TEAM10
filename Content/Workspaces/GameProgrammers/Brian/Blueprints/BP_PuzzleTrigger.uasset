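; BP_PuzzleTrigger is a damageable puzzle actor that unlocks only when hit by the player holding a specific weapon.
; On damage it compares the player character's current weapon index with its own WeaponIndex, then fires LockTriggered and destroys itself on a match.
; On a mismatch it heals back to max health through its GP_Health component, printing a debug message if that fails.
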(event `self.GP_Health.OnDamage`
  (bind _gp_health (`self.GP_Health`))
  (bind _asbp_brian_player_test_character (cast `/Game/Workspaces/GameProgrammers/Brian/Blueprints/BP_BrianPlayerTestCharacter` (`GameplayStatics.GetPlayerCharacter` 0)))
  (if (== (`/Game/Workspaces/GameProgrammers/Doruk/Blueprints/BP_BackupDorukCharacter.CurrentWeaponIndex` _asbp_brian_player_test_character) (`self.WeaponIndex`))
    (`self.LockTriggered`)
    (`self.K2_DestroyActor`)
    (else
      (bind _returnvalue (`GP_HealthComponent.TryToAddHealth` _gp_health (- (`GP_HealthComponent.MaxHealth` _gp_health) (`GP_HealthComponent.GetHealth` _gp_health))))
      (if (not _returnvalue)
        (`KismetSystemLibrary.PrintString` "Couldn't restore HP to the PuzzleTrigger!" true true (struct :`R` 0.257671 :`G` 0.103803 :`B` 1.0 :`A` 1.0))))))

(fn `UserConstructionScript`)