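; BP_SingleDoor is a single swinging door that opens when the local player's pawn enters its TV_Door trigger.
; The overlap plays a timeline whose curve lerps the door mesh's relative yaw from zero to DoorOpenAngle.
; The end-overlap handler checks for the player but does nothing, so the door never closes.
; BeginPlay applies the configurable DoorStaticMesh, leaving the construction script empty.
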(event `self.TV_Door.OnComponentBeginOverlap`
  (params (OverlappedComponent :type "PrimitiveComponent Object Reference") (OtherActor :type "Actor Object Reference") (OtherComp :type "PrimitiveComponent Object Reference") (OtherBodyIndex :type Integer) (bFromSweep :type Boolean) (SweepResult :type "HitResult Structure (by ref)"))
  (if (== OtherActor (`GameplayStatics.GetPlayerPawn` 0))
    (bind (_direction _openclosedoorcurve) (`Timeline|TL_OpenCloseDoor`)
      (:`Update`
        (`SceneComponent.K2_SetRelativeRotation` (`self.SM_Door_Double_A_Solo`) (`KismetMathLibrary.MakeRotator` 0.0 0.0 (`KismetMathLibrary.Lerp` 0.0 (`self.DoorOpenAngle`) _openclosedoorcurve)) false false)))))

(event `self.TV_Door.OnComponentEndOverlap`
  (params (OverlappedComponent :type "PrimitiveComponent Object Reference") (OtherActor :type "Actor Object Reference") (OtherComp :type "PrimitiveComponent Object Reference") (OtherBodyIndex :type Integer))
  (if (== (`GameplayStatics.GetPlayerPawn` 0) OtherActor)
    _))

(event `self.ReceiveBeginPlay`
  (`StaticMeshComponent.SetStaticMesh` (`self.SM_Door_Double_A_Solo`) (`self.DoorStaticMesh`)))

(fn `UserConstructionScript`)