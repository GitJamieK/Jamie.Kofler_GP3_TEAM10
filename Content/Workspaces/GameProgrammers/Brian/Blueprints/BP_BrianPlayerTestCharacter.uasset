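; Test player character Blueprint that ties health, healing and aiming to the HUD and camera.
; GPHealth changes update the health text and run a timeline that blends saturation and vignette on the follow camera, while death is passed to GP_GameModeBase.
; F spends an inventory health pack to heal, and T applies test self-damage.
; AimWeapon switches walk speed and orient-to-movement, fading the crosshair and ammo switcher widgets.
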(event `self.ReceiveBeginPlay`
  (`parent.ReceiveBeginPlay`)
  (add `GP_HealthComponent.OnDeath` (`self.GP_Health`) (delegate `OnDeath_Event`)))

(event `OnDeath_Event`
  (bind _asgp_game_mode_base (cast `GP_GameModeBase` (`GameplayStatics.GetGameMode`)))
  (`GP_GameModeBase.HandleDeathState` _asgp_game_mode_base))

(event `self.GP_Health.OnHealthChanged`
  (params (Health :type "Float (single-precision)") (Delta :type "Float (single-precision)"))
  (bind _returnvalue (`GP_HealthComponent.GetHealthPercent` (`self.GP_Health`)))
  (bind ((`ColorSaturation` _colorsaturation) (`VignetteIntensity` _vignetteintensity)) (break `PostProcessSettings` (`CameraComponent.PostProcessSettings` (`self.FollowCamera`))))
  ; Logic of Post Processing Changes Based on HP
  (`self.ChangeHPBarText` Health)
  (bind (_direction _smoothfloatcurve) (`Timeline|TL_SmoothPostProcess` :!via `PlayFromStart`)
    (:`Update`
      (set `CameraComponent.PostProcessSettings` (make `PostProcessSettings` :`ColorSaturation` (`KismetMathLibrary.MakeVector4` 1.0 1.0 1.0 (`KismetMathLibrary.Lerp` (`.W` (`KismetMathLibrary.BreakVector4` _colorsaturation)) _returnvalue _smoothfloatcurve)) :`VignetteIntensity` (`KismetMathLibrary.Lerp` _vignetteintensity (+ (- 1.0 _returnvalue) 0.4) _smoothfloatcurve)) (`self.FollowCamera`)))))

(event `Key|T`
  (params (Key :type "Key Structure"))
  ;[1 0 0 0.5] Testing
  (:`Pressed`
    (`GameplayStatics.ApplyDamage` self 10.0)))

(event `Key|F`
  (params (Key :type "Key Structure"))
  ; Heal Logic
  (:`Pressed`
    (if (`GP_HealthComponent.IsHealthFull` (`self.GP_Health`))
      (`KismetSystemLibrary.PrintString` "You're Full HP!!" true true (struct :`R` 1.0 :`B` 0.139721 :`A` 1.0))
      (else
        (bind _returnvalue (`GP_InventoryComponent.UseItem` (`self.GP_Inventory`) "HealthPack"))
        (if _returnvalue
          (`GP_HealthComponent.TryToAddHealth` (`self.GP_Health`) 50.0)
          (else
            (`KismetSystemLibrary.PrintString` "No Health Packs!" true true (struct :`R` 1.0 :`G` 0.082806 :`B` 0.072858 :`A` 1.0))))))))

(fn `AimWeapon`
  (params (bIsAiming :type Boolean))
  (bind _charactermovement (`self.CharacterMovement`))
  (bind _charactermovement_2 (`self.CharacterMovement`))
  (if bIsAiming
    (`self.PlayFadeInAnim`)
    (set `CharacterMovementComponent.MaxWalkSpeed` (`self.PlayerAimingSpeed`) _charactermovement_2)
    (set `CharacterMovementComponent.bOrientRotationToMovement` false _charactermovement_2)
    (else
      (`self.PlayFadeOutAnim`)
      (set `CharacterMovementComponent.MaxWalkSpeed` (`self.PlayerWalkingSpeed`) _charactermovement)
      (set `CharacterMovementComponent.bOrientRotationToMovement` true _charactermovement)))
  (return))

(fn `ChangeHPBarText`
  (params (Health :type "Float (double-precision)"))
  (bind _asgame_hud (cast `/Game/UI/GameHUD` (`PlayerController.GetHUD` (`GameplayStatics.GetPlayerController` 0))))
  (set `TextBlock.Text` (`|FormatText` "Health: {Health}" Health) (`/Game/UI/WBP_HealthBar.HPText` (`/Game/UI/GameHUD.UI_HealthBarRef` _asgame_hud))))

(fn `PlayFadeInAnim`
  (bind _asgame_hud (cast `/Game/UI/GameHUD` (`PlayerController.GetHUD` (`GameplayStatics.GetPlayerController` 0))))
  (bind _ui_ammoswitcherref (`/Game/UI/GameHUD.UI_AmmoSwitcherRef` _asgame_hud))
  (`UserWidget.PlayAnimation` _ui_ammoswitcherref (`/Game/UI/AmmoUI/WBP_AmmoSwitcher.Fade` _ui_ammoswitcherref) 0.0 1 "Forward" 1.0 false)
  (bind _ui_crosshairref (`/Game/UI/GameHUD.UI_CrosshairRef` _asgame_hud))
  (`UserWidget.PlayAnimation` _ui_crosshairref (`/Game/UI/WBP_Crosshair.Fade` _ui_crosshairref) 0.0 1 "Forward" 1.0 false))

(fn `PlayFadeOutAnim`
  (bind _asgame_hud (cast `/Game/UI/GameHUD` (`PlayerController.GetHUD` (`GameplayStatics.GetPlayerController` 0))))
  (bind _ui_ammoswitcherref (`/Game/UI/GameHUD.UI_AmmoSwitcherRef` _asgame_hud))
  (`UserWidget.PlayAnimation` _ui_ammoswitcherref (`/Game/UI/AmmoUI/WBP_AmmoSwitcher.Fade` _ui_ammoswitcherref) 0.0 1 "Reverse" 1.0 false)
  (bind _ui_crosshairref (`/Game/UI/GameHUD.UI_CrosshairRef` _asgame_hud))
  (`UserWidget.PlayAnimation` _ui_crosshairref (`/Game/UI/WBP_Crosshair.Fade` _ui_crosshairref) 0.0 1 "Reverse" 1.0 false))

(fn `UserConstructionScript`
  (`parent.UserConstructionScript`))