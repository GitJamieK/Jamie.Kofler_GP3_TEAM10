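; BP_FireDoor is a puzzle door that rises once all of its assigned lock trigger actors have fired.
; On BeginPlay it binds to each PuzzleTriggerActors lock event, and CheckLocks counts triggers until the count matches the array length.
; Opening waits briefly, plays a metal gate sound, then runs a timeline that lifts the root, re-reading its current world location as the Lerp base every update.
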(event `self.ReceiveBeginPlay`
  (`self.BindLockTriggered`))

(event `CE_OpenDoor`
  (bind _defaultsceneroot (`self.DefaultSceneRoot`))
  (bind (_returnvalue_x _returnvalue_y _returnvalue_z) (`KismetMathLibrary.BreakVector` (`SceneComponent.K2_GetComponentLocation` _defaultsceneroot)))
  (`KismetSystemLibrary.Delay` 0.8)
  (bind _returnvalue (`FMODBlueprintStatics.PlayEventAtLocation` "/Game/FMOD/Events/Environment/ObjectInteractions/MetalGate.MetalGate" (`self.GetTransform`)))
  (`FMODBlueprintStatics.EventInstanceRelease` _returnvalue)
  (bind (_direction _openclosedoorcurve) (`Timeline|TL_OpenDoor`)
    (:`Update`
      (`SceneComponent.K2_SetRelativeTransform` _defaultsceneroot (`KismetMathLibrary.MakeTransform` (`KismetMathLibrary.MakeVector` _returnvalue_x _returnvalue_y (`KismetMathLibrary.Lerp` _returnvalue_z (+ _returnvalue_z 250.0) _openclosedoorcurve)) (`SceneComponent.K2_GetComponentRotation` _defaultsceneroot)) false false))))

(fn `BindLockTriggered`
  (for _array_element (`self.PuzzleTriggerActors`)
    (add `/Game/Workspaces/GameProgrammers/Brian/Blueprints/BP_FirePuzzleTrigger.LockTriggered` _array_element (`|CreateDelegate` :!event `CheckLocks`))))

(fn `CheckLocks`
  (bind _result (`/Engine/EditorBlueprintResources/StandardMacros.IncrementInt` (`self.LocksTriggered`))
    (:`  `
      (if (== _result (`KismetArrayLibrary.Array_Length` (`self.PuzzleTriggerActors`)))
        (`self.CE_OpenDoor`)))))

(fn `UserConstructionScript`)