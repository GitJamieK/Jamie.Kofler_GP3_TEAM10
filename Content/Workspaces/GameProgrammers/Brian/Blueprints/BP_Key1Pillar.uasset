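; A key pillar Blueprint that accepts a Key1 item from the player, with its item type set to Key1 in the construction script.
; Pressing E tries to use Key1 from the player's inventory, printing a debug message on failure.
; On success it switches the statue VFX material to placed, calls CallUsedKey, records its PillarID in saved game data and, if that data is valid, plays a placement sound event.
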(event `Key|E`
  (params (Key :type "Key Structure"))
  (:`Pressed`
    (bind _asbp_brian_player_test_character (cast `/Game/Workspaces/GameProgrammers/Brian/Blueprints/BP_BrianPlayerTestCharacter` (`GameplayStatics.GetPlayerCharacter` 0)))
    (bind _returnvalue (`GP_InventoryComponent.UseItem` (`/Game/Workspaces/GameProgrammers/Doruk/Blueprints/BP_BackupDorukCharacter.GP_Inventory` _asbp_brian_player_test_character) "key1"))
    (if _returnvalue
      (`MaterialInstanceDynamic.SetScalarParameterValue` (`self.StatueVFX`) "0=NO STATUE, 1=PLACED STATUE" 1.0)
      (`self.UsedKey` "key1")
      (bind _savegamedata (message `/Game/Workspaces/GameProgrammers/Brian/SaveGame/BPI_SaveGame.GetSavedGameData` (`GameplayStatics.GetGameInstance`)))
      (`/Engine/EditorBlueprintResources/StandardMacros.IsValid` _savegamedata
        (:`Is Valid`
          (`BlueprintMapLibrary.Map_Add` (`/Game/Workspaces/GameProgrammers/Brian/SaveGame/BP_SaveGame.PillarsWithStatues` _savegamedata) (`self.PillarID`) true)
          (bind _returnvalue_2 (`FMODBlueprintStatics.PlayEventAtLocation` "/Game/FMOD/Events/Environment/ObjectInteractions/PlaceObject.PlaceObject" (`self.GetTransform`)))
          (`FMODBlueprintStatics.EventInstanceRelease` _returnvalue_2)))
      (else
        (`KismetSystemLibrary.PrintString` "You don't have the requiered key!")))))

(fn `UserConstructionScript`
  (`parent.UserConstructionScript`)
  (set `self.Item Type` "key1"))