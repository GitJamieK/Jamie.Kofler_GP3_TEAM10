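; BP_2DSoundEventFMOD is an overlap-triggered actor that plays a 2D FMOD sound event while the player is inside it.
; When the first player pawn begins overlapping, it plays the EventFMOD event in 2D and stores the returned instance.
; When that pawn stops overlapping, it stops and releases the stored instance.
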(event `self.ReceiveActorBeginOverlap`
  (params (OtherActor :type "Actor Object Reference"))
  (if (== OtherActor (`GameplayStatics.GetPlayerPawn` 0))
    (bind _returnvalue (`FMODBlueprintStatics.PlayEvent2D` (`self.EventFMOD`)))
    (set `self.Event` _returnvalue)))

(event `self.ReceiveActorEndOverlap`
  (params (OtherActor :type "Actor Object Reference"))
  (if (== OtherActor (`GameplayStatics.GetPlayerPawn` 0))
    (`FMODBlueprintStatics.EventInstanceStop` (`self.Event`) true)))

(fn `UserConstructionScript`)