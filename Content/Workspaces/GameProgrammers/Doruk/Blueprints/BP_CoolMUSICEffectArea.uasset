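; A trigger-area Blueprint in a programmer workspace that plays moonlight music when the player enters it.
; On begin overlap, it checks that the actor is player pawn 0 and that ShouldDoEffect is set, then plays MoonlightMusic as a 2D event.
; When the player leaves, it clears ShouldDoEffect, so later entries do not retrigger the music.
; Nothing here stops the music or resets the flag.
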(event `self.ReceiveActorBeginOverlap`
  (params (OtherActor :type "Actor Object Reference"))
  (if (and (== OtherActor (`GameplayStatics.GetPlayerPawn` 0)) (`self.ShouldDoEffect`))
    (`FMODBlueprintStatics.PlayEvent2D` "/Game/FMOD/Events/Music/MoonlightMusic.MoonlightMusic")))

(event `self.ReceiveActorEndOverlap`
  (params (OtherActor :type "Actor Object Reference"))
  (if (== OtherActor (`GameplayStatics.GetPlayerPawn` 0))
    (set `self.ShouldDoEffect` false)))

(fn `UserConstructionScript`)