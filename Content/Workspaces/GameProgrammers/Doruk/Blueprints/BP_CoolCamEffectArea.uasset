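; BP_CoolCamEffectArea is an overlap area that shifts the player's camera while they are inside it.
; On entry, the CamEffect timeline lerps BP_BackupDorukCharacter's SpringArm socket offset from its starting value to a hardcoded offset.
; On exit, it reverses the timeline and clears ShouldDoEffect, which this graph never resets, so later entries do not replay the effect.
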(event `self.ReceiveActorBeginOverlap`
  (params (OtherActor :type "Actor Object Reference"))
  (if (and (== OtherActor (`GameplayStatics.GetPlayerPawn` 0)) (`self.ShouldDoEffect`))
    (bind _asbp_backup_doruk_character (cast `/Game/Workspaces/GameProgrammers/Doruk/Blueprints/BP_BackupDorukCharacter` OtherActor))
    (bind (_direction _transition) (`Timeline|CamEffect` :!label _label)
      (:`Update`
        (bind (_startingsocketoffset_x _startingsocketoffset_y _startingsocketoffset_z) (`KismetMathLibrary.BreakVector` (`/Game/Workspaces/GameProgrammers/Doruk/Blueprints/BP_BackupDorukCharacter.StartingSocketOffset` _asbp_backup_doruk_character)))
        (set `SpringArmComponent.SocketOffset` (`KismetMathLibrary.MakeVector` (`KismetMathLibrary.Lerp` _startingsocketoffset_x -288.0 _transition) (`KismetMathLibrary.Lerp` _startingsocketoffset_y 95.0 _transition) (`KismetMathLibrary.Lerp` _startingsocketoffset_z 135.0 _transition)) (`/Game/Workspaces/GameProgrammers/Doruk/Blueprints/BP_BackupDorukCharacter.SpringArm` _asbp_backup_doruk_character))))))

(event `self.ReceiveActorEndOverlap`
  (params (OtherActor :type "Actor Object Reference"))
  (if (== OtherActor (`GameplayStatics.GetPlayerPawn` 0))
    (set `self.ShouldDoEffect` false)
    (goto _label :!via `Reverse`)))

(fn `UserConstructionScript`)