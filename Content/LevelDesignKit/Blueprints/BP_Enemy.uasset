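; BP_Enemy is a level design kit enemy that takes damage when something overlaps its damage radius or its Hit event fires.
; Each hit shows pain text, plays a grunt and subtracts Damage from Life, hiding the text afterward if it survives.
; When Life equals exactly zero, a timeline tips the mesh over and shows the death line, then text, collision and body are switched off after a delay.
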(event `self.ReceiveBeginPlay`
  ;[1 1 1] Start - Setting Variables
  (`SceneComponent.ToggleVisibility` (`self.TextRender`) false)
  (bind _output_get (set `self.Life` (`self.Life`)))
  (`KismetSystemLibrary.PrintString` (`KismetStringLibrary.Conv_DoubleToString` _output_get))
  (bind _output_get_2 (set `self.Damage` (`self.Damage`)))
  (`KismetSystemLibrary.PrintString` (`KismetStringLibrary.Conv_DoubleToString` _output_get_2)))

(event `self.TV_Damage_Radius.OnComponentBeginOverlap`
  (params (OverlappedComponent :type "PrimitiveComponent Object Reference") (OtherActor :type "Actor Object Reference") (OtherComp :type "PrimitiveComponent Object Reference") (OtherBodyIndex :type Integer) (bFromSweep :type Boolean) (SweepResult :type "HitResult Structure (by ref)"))
  ;[1 1 1] Check if Hit or Close
  ;[1 1 1] If Enemy Alive, Cause Damage
  (if (not (`self.Enemy Dead`)) :!label _label
    (`|ExecutionSequence`
      (:`then_0`
        (`SceneComponent.SetVisibility` (`self.TextRender`) true false)
        (bind _output_get (set `self.Life` (- (`self.Life`) (`self.Damage`))))
        (`KismetSystemLibrary.PrintString` (`KismetStringLibrary.Conv_DoubleToString` _output_get))
        (if (== 0.0 (`self.Life`))
          ;[1 1 1] Trigger Death Sequence
          (bind (_direction _bodyfall) (`Timeline|BodyFall`)
            (:`Update`
              (`SceneComponent.K2_SetRelativeRotation` (`self.SM_Pose1B_AimGunRiffle`) (`KismetMathLibrary.MakeRotator` 0.0 (`KismetMathLibrary.Lerp` 0.0 80.0 _bodyfall)) false false)
              (`TextRenderComponent.K2_SetText` (`self.TextRender`) (`self.Death Line`))
              (set `self.Enemy Dead` true)
              (`KismetSystemLibrary.Delay` 2.0)
              (`SceneComponent.SetVisibility` (`self.TextRender`) false false)
              (`PrimitiveComponent.SetCollisionEnabled` (`self.TV_Damage_Radius`) "NoCollision")
              (`PrimitiveComponent.SetCollisionEnabled` (`self.SM_Pose1B_AimGunRiffle`) "NoCollision")
              (`SceneComponent.ToggleVisibility` (`self.SM_Pose1B_AimGunRiffle`) false)))
          (else
            ;[1 1 1] Visual Feedback on Damage
            (`KismetSystemLibrary.PrintString` "Enemy is Still Alive")
            (`KismetSystemLibrary.Delay` 0.5)
            (`SceneComponent.SetVisibility` (`self.TextRender`) false false))))
      (:`then_1`
        (`GameplayStatics.PlaySound2D` "/Game/LevelDesignKit/Audio/SFX_EnemyGrunt_03.SFX_EnemyGrunt_03" 1.0 1.0 0.0 null null)))))

(event `self.ReceiveHit`
  (params (MyComp :type "PrimitiveComponent Object Reference") (Other :type "Actor Object Reference") (OtherComp :type "PrimitiveComponent Object Reference") (bSelfMoved :type Boolean) (HitLocation :type "Vector Structure") (HitNormal :type "Vector Structure") (NormalImpulse :type "Vector Structure") (Hit :type "HitResult Structure (by ref)"))
  ;[1 1 1] Check if Hit or Close
  (goto _label))

(fn `UserConstructionScript`)