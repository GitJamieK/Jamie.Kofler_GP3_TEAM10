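; BP_FallingStalactites_6m is a level design hazard prop: two stalactites that fall when something overlaps its trigger volume.
; The TV_RocksFall overlap plays a 2D rock-fall sound and starts two timelines, each driving one mesh's relative location without sweep or physics.
; The Fallen flag, set during the first timeline's update, blocks later triggers, and the overlapping actor is not filtered.
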(event `self.TV_RocksFall.OnComponentBeginOverlap`
  (params (OverlappedComponent :type "PrimitiveComponent Object Reference") (OtherActor :type "Actor Object Reference") (OtherComp :type "PrimitiveComponent Object Reference") (OtherBodyIndex :type Integer) (bFromSweep :type Boolean) (SweepResult :type "HitResult Structure (by ref)"))
  ;[1 1 1] Enter Trigger Rocks Fall
  (if (not (`self.Fallen`))
    (`GameplayStatics.PlaySound2D` "/Game/LevelDesignKit/Audio/SFX_RockFaling.SFX_RockFaling" 1.0 1.0 0.0 null null)
    (`|ExecutionSequence`
      (:`then_0`
        (bind (_direction _newtrack_1) (`Timeline|Rock1_Fall`)
          (:`Update`
            (`SceneComponent.K2_SetRelativeLocation` (`self.SM_Stalactite02`) _newtrack_1 false false)
            (set `self.Fallen` true))))
      (:`then_1`
        (bind (_direction_2 _newtrack_1_2) (`Timeline|Timeline`)
          (:`Update`
            (`SceneComponent.K2_SetRelativeLocation` (`self.SM_Stalactite01`) _newtrack_1_2 false false)))))))

(fn `UserConstructionScript`)